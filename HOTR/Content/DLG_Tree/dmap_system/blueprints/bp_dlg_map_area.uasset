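; Map area actor for the DLG minimap system, defining a bounded world region captured by a scene capture into a render target.
; RefreshValues fits the capture and preview components to bounds, angle and yaw; Tick optionally recaptures and copies camera yaw.
; Helpers convert between world and normalized, yaw-rotated map coordinates, then into zoomed, edge-clamped widget positions.
; Actor tags mark map ID and active state, while SetMap links the widget that receives registered icons.
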(event `self.ReceiveBeginPlay`
  ;[1 1 1] Map system beginplay is here.
  (`self.refresh_values`)
  (`self.init_map` (`self.map_id`))
  (`self.set_origin` (`self.K2_GetActorLocation`) (`self.map_bounds`)))

(event `self.ReceiveTick`
  (params (DeltaSeconds :type "Float (single-precision)"))
  ;[1 1 1] Map system beginplay is here.
  (`|ExecutionSequence`
    (:`then_0`
      (if (`self.use_capture`)
        (`SceneCaptureComponent2D.CaptureScene` (`self.map_capture`))))
    (:`then_1`
      (if (`self.rotate_player`)
        (set `self.capture_yaw` (.yaw (`PlayerCameraManager.GetCameraRotation` (`GameplayStatics.GetPlayerCameraManager` 0))))))))

(fn `clamp_local_borders`
  (params (map_loc :type "Vector Structure") (map_size :type "Vector Structure") (map_offset :type "Vector Structure") (map_zoom :type "Float (double-precision)") (icon_size :type "Float (double-precision)"))
  (returns (clamped_value :type "Vector Structure") (unclamped_value :type "Vector Structure"))
  (locals (local_vec :type "Vector Structure") (local_map_size :type "Vector Structure") (local_icon_size :type "Float (double-precision)") (local_offset :type "Vector Structure") (local_zoom :type "Float (double-precision)"))
  (bind _x (.x (`local.local_map_size`)))
  (bind _y (.y (`local.local_map_size`)))
  (bind _z (.z (`local.local_map_size`)))
  (bind _x_2 (.x (`local.local_vec`)))
  (bind _y_2 (.y (`local.local_vec`)))
  (bind _z_2 (.z (`local.local_vec`)))
  (bind _returnvalue (+ _x_2 (`local.local_icon_size`)))
  (bind _returnvalue_2 (+ _z_2 (`local.local_icon_size`)))
  (bind _returnvalue_3 (+ _y_2 (`local.local_icon_size`)))
  ;[1 1 1] Clamp borders logic.
  (set `local.local_vec` map_loc)
  (set `local.local_map_size` map_size)
  (set `local.local_offset` map_offset)
  (set `local.local_zoom` map_zoom)
  (set `local.local_icon_size` icon_size)
  (return (`KismetMathLibrary.MakeVector` (+ _x_2 (`KismetMathLibrary.SelectFloat` (- (`KismetMathLibrary.Abs` _x_2) (`local.local_icon_size`)) (`KismetMathLibrary.SelectFloat` (- (- _x _x_2) (`local.local_icon_size`)) 0.0 (> _returnvalue _x)) (< _returnvalue 0.0))) (+ _y_2 (`KismetMathLibrary.SelectFloat` (- (`KismetMathLibrary.Abs` _y_2) (`local.local_icon_size`)) (`KismetMathLibrary.SelectFloat` (- (- _y _y_2) (`local.local_icon_size`)) 0.0 (> _returnvalue_3 _y)) (< _returnvalue_3 0.0))) (+ _z_2 (`KismetMathLibrary.SelectFloat` (- (`KismetMathLibrary.Abs` _z_2) (`local.local_icon_size`)) (`KismetMathLibrary.SelectFloat` (- (- _z _z_2) (`local.local_icon_size`)) 0.0 (> _returnvalue_2 _z)) (< _returnvalue_2 0.0)))) (`local.local_vec`)))

(fn `convert_exponent_to_world`
  (params (exponent_loc :type "Vector Structure"))
  (returns (world_loc :type "Vector Structure"))
  (locals (local_input_loc :type "Vector Structure"))
  ;[1 1 1] Convert input location to map location.
  (set `local.local_input_loc` exponent_loc)
  (return (- (`KismetMathLibrary.MakeVector` (`KismetMathLibrary.MapRangeUnclamped` (.x (`KismetMathLibrary.LessLess_VectorRotator` (`local.local_input_loc`) (`KismetMathLibrary.MakeRotator` 0.0 0.0 (`self.capture_yaw`)))) 1.0 -1.0 (.x (`KismetMathLibrary.MakeVector` (- (.x (`self.map_origin`)) (/ (.x (`self.map_bounds`)) 2.0)) (- (.y (`self.map_origin`)) (/ (.y (`self.map_bounds`)) 2.0)) (- (.z (`self.map_origin`)) (/ (.z (`self.map_bounds`)) 2.0)))) (.x (`KismetMathLibrary.MakeVector` (+ (.x (`self.map_origin`)) (/ (.x (`self.map_bounds`)) 2.0)) (+ (.y (`self.map_origin`)) (/ (.y (`self.map_bounds`)) 2.0)) (+ (.z (`self.map_origin`)) (/ (.z (`self.map_bounds`)) 2.0))))) (`KismetMathLibrary.MapRangeUnclamped` (.y (`KismetMathLibrary.LessLess_VectorRotator` (`local.local_input_loc`) (`KismetMathLibrary.MakeRotator` 0.0 0.0 (`self.capture_yaw`)))) -1.0 1.0 (.y (`KismetMathLibrary.MakeVector` (- (.x (`self.map_origin`)) (/ (.x (`self.map_bounds`)) 2.0)) (- (.y (`self.map_origin`)) (/ (.y (`self.map_bounds`)) 2.0)) (- (.z (`self.map_origin`)) (/ (.z (`self.map_bounds`)) 2.0)))) (.y (`KismetMathLibrary.MakeVector` (+ (.x (`self.map_origin`)) (/ (.x (`self.map_bounds`)) 2.0)) (+ (.y (`self.map_origin`)) (/ (.y (`self.map_bounds`)) 2.0)) (+ (.z (`self.map_origin`)) (/ (.z (`self.map_bounds`)) 2.0))))) (`KismetMathLibrary.MapRangeUnclamped` (.z (`KismetMathLibrary.LessLess_VectorRotator` (`local.local_input_loc`) (`KismetMathLibrary.MakeRotator` 0.0 0.0 (`self.capture_yaw`)))) -1.0 1.0 (.z (`KismetMathLibrary.MakeVector` (- (.x (`self.map_origin`)) (/ (.x (`self.map_bounds`)) 2.0)) (- (.y (`self.map_origin`)) (/ (.y (`self.map_bounds`)) 2.0)) (- (.z (`self.map_origin`)) (/ (.z (`self.map_bounds`)) 2.0)))) (.z (`KismetMathLibrary.MakeVector` (+ (.x (`self.map_origin`)) (/ (.x (`self.map_bounds`)) 2.0)) (+ (.y (`self.map_origin`)) (/ (.y (`self.map_bounds`)) 2.0)) (+ (.z (`self.map_origin`)) (/ (.z (`self.map_bounds`)) 2.0)))))) (- (`self.map_origin`) (`self.K2_GetActorLocation`)))))

(fn `convert_map_offset`
  (params (map_offset :type "Vector Structure") (owner_location :type "Vector Structure") (map_size :type "Float (double-precision)" :default 1024.0) (map_zoom :type "Float (double-precision)" :default 1.0))
  (returns (base_offset :type "Vector Structure"))
  (locals (local_zoom :type "Float (double-precision)") (local_offset :type "Vector Structure" :default (0.0 0.0 0.0)) (local_size :type "Float (double-precision)"))
  (bind _local_size (`local.local_size`))
  (bind _returnvalue (/ _local_size 2.0))
  (bind _returnvalue_2 (`KismetMathLibrary.MapRangeUnclamped` (`local.local_zoom`) 1.0 2.0 _returnvalue _local_size))
  (bind _returnvalue_3 (`KismetMathLibrary.MapRangeUnclamped` (`local.local_zoom`) 1.0 2.0 _returnvalue _local_size))
  (bind _returnvalue_4 (`KismetMathLibrary.Abs` (`KismetMathLibrary.GridSnap_Float` (`self.capture_yaw`) 45.0)))
  (bind _returnvalue_5 (/ (* (`local.local_size`) (`local.local_zoom`)) 2.0))
  (bind _returnvalue_6 (`KismetMathLibrary.MapRangeUnclamped` (`local.local_zoom`) 1.0 2.0 _returnvalue _local_size))
  (bind _returnvalue_7 (* _returnvalue_5 -1.0))
  (bind _returnvalue_8 (`KismetMathLibrary.MapRangeUnclamped` (`local.local_zoom`) 0.97 2.0 (/ (`local.local_size`) 2.0) (/ (`local.local_size`) (`KismetMathLibrary.SelectFloat` 0.5 1.0 (or (== _returnvalue_4 45.0) (== _returnvalue_4 135.0))))))
  (bind _returnvalue_9 (* _returnvalue_8 -1.0))
  ;[1 1 1] Calculate map offset with zoom.
  (set `local.local_offset` map_offset)
  (set `local.local_size` map_size)
  (set `local.local_zoom` map_zoom)
  (return (`KismetMathLibrary.MakeVector` (`KismetMathLibrary.FClamp` (.x (`KismetMathLibrary.SelectVector` (`KismetMathLibrary.MakeVector` (`KismetMathLibrary.MapRangeUnclamped` (.x (`self.convert_world_to_exponent` owner_location)) -1.0 1.0 _returnvalue_5 _returnvalue_7) (`KismetMathLibrary.MapRangeUnclamped` (.y (`self.convert_world_to_exponent` owner_location)) -1.0 1.0 _returnvalue_5 _returnvalue_7) (`KismetMathLibrary.MapRangeUnclamped` (.z (`self.convert_world_to_exponent` owner_location)) -1.0 1.0 _returnvalue_5 _returnvalue_7)) (`KismetMathLibrary.MakeVector` (`KismetMathLibrary.MapRangeUnclamped` (.x (`local.local_offset`)) -1.0 1.0 _returnvalue_6 (* _returnvalue_6 -1.0)) (`KismetMathLibrary.MapRangeUnclamped` (.y (`local.local_offset`)) -1.0 1.0 _returnvalue_3 (* _returnvalue_3 -1.0)) (`KismetMathLibrary.MapRangeClamped` (.z (`local.local_offset`)) -1.0 1.0 _returnvalue_2 (* _returnvalue_2 -1.0))) (== (`local.local_offset`) (0.0 0.0 0.0)))) _returnvalue_9 _returnvalue_8) (`KismetMathLibrary.FClamp` (.y (`KismetMathLibrary.SelectVector` (`KismetMathLibrary.MakeVector` (`KismetMathLibrary.MapRangeUnclamped` (.x (`self.convert_world_to_exponent` owner_location)) -1.0 1.0 _returnvalue_5 _returnvalue_7) (`KismetMathLibrary.MapRangeUnclamped` (.y (`self.convert_world_to_exponent` owner_location)) -1.0 1.0 _returnvalue_5 _returnvalue_7) (`KismetMathLibrary.MapRangeUnclamped` (.z (`self.convert_world_to_exponent` owner_location)) -1.0 1.0 _returnvalue_5 _returnvalue_7)) (`KismetMathLibrary.MakeVector` (`KismetMathLibrary.MapRangeUnclamped` (.x (`local.local_offset`)) -1.0 1.0 _returnvalue_6 (* _returnvalue_6 -1.0)) (`KismetMathLibrary.MapRangeUnclamped` (.y (`local.local_offset`)) -1.0 1.0 _returnvalue_3 (* _returnvalue_3 -1.0)) (`KismetMathLibrary.MapRangeClamped` (.z (`local.local_offset`)) -1.0 1.0 _returnvalue_2 (* _returnvalue_2 -1.0))) (== (`local.local_offset`) (0.0 0.0 0.0)))) _returnvalue_9 _returnvalue_8) (`KismetMathLibrary.FClamp` (.z (`KismetMathLibrary.SelectVector` (`KismetMathLibrary.MakeVector` (`KismetMathLibrary.MapRangeUnclamped` (.x (`self.convert_world_to_exponent` owner_location)) -1.0 1.0 _returnvalue_5 _returnvalue_7) (`KismetMathLibrary.MapRangeUnclamped` (.y (`self.convert_world_to_exponent` owner_location)) -1.0 1.0 _returnvalue_5 _returnvalue_7) (`KismetMathLibrary.MapRangeUnclamped` (.z (`self.convert_world_to_exponent` owner_location)) -1.0 1.0 _returnvalue_5 _returnvalue_7)) (`KismetMathLibrary.MakeVector` (`KismetMathLibrary.MapRangeUnclamped` (.x (`local.local_offset`)) -1.0 1.0 _returnvalue_6 (* _returnvalue_6 -1.0)) (`KismetMathLibrary.MapRangeUnclamped` (.y (`local.local_offset`)) -1.0 1.0 _returnvalue_3 (* _returnvalue_3 -1.0)) (`KismetMathLibrary.MapRangeClamped` (.z (`local.local_offset`)) -1.0 1.0 _returnvalue_2 (* _returnvalue_2 -1.0))) (== (`local.local_offset`) (0.0 0.0 0.0)))) _returnvalue_9 _returnvalue_8))))

(fn `convert_map_value`
  (params (exponent_loc :type "Vector Structure") (map_size :type "Vector Structure") (map_offset :type "Vector Structure") (map_zoom :type "Float (double-precision)") (icon_size :type "Float (double-precision)"))
  (returns (clamped_value :type "Vector Structure") (unclamped_value :type "Vector Structure"))
  (locals (local_location :type "Vector Structure") (local_zoom :type "Float (double-precision)") (local_size :type "Vector Structure") (local_offset :type "Vector Structure") (local_icon :type "Float (double-precision)"))
  (bind _returnvalue (/ (`local.local_size`) 2.0))
  ;[1 1 1] Convert map value to map location.
  (set `local.local_location` exponent_loc)
  (set `local.local_size` map_size)
  (set `local.local_offset` map_offset)
  (set `local.local_zoom` map_zoom)
  (set `local.local_icon` icon_size)
  (bind (_clamped_value _unclamped_value) (`self.clamp_local_borders` (- (- (`KismetMathLibrary.MakeVector` (+ (.x (* (`KismetMathLibrary.MakeVector` (`KismetMathLibrary.MapRangeUnclamped` (.x (`local.local_location`)) -1.0 1.0 0.0 (.x (`local.local_size`))) (`KismetMathLibrary.MapRangeUnclamped` (.y (`local.local_location`)) -1.0 1.0 0.0 (.y (`local.local_size`))) (`KismetMathLibrary.MapRangeUnclamped` (.z (`local.local_location`)) -1.0 1.0 0.0 (.z (`local.local_size`)))) (`local.local_zoom`))) (.x (`local.local_offset`))) (+ (.y (* (`KismetMathLibrary.MakeVector` (`KismetMathLibrary.MapRangeUnclamped` (.x (`local.local_location`)) -1.0 1.0 0.0 (.x (`local.local_size`))) (`KismetMathLibrary.MapRangeUnclamped` (.y (`local.local_location`)) -1.0 1.0 0.0 (.y (`local.local_size`))) (`KismetMathLibrary.MapRangeUnclamped` (.z (`local.local_location`)) -1.0 1.0 0.0 (.z (`local.local_size`)))) (`local.local_zoom`))) (.y (`local.local_offset`))) (+ (.z (* (`KismetMathLibrary.MakeVector` (`KismetMathLibrary.MapRangeUnclamped` (.x (`local.local_location`)) -1.0 1.0 0.0 (.x (`local.local_size`))) (`KismetMathLibrary.MapRangeUnclamped` (.y (`local.local_location`)) -1.0 1.0 0.0 (.y (`local.local_size`))) (`KismetMathLibrary.MapRangeUnclamped` (.z (`local.local_location`)) -1.0 1.0 0.0 (.z (`local.local_size`)))) (`local.local_zoom`))) (.z (`local.local_offset`)))) (- (* _returnvalue (`local.local_zoom`)) _returnvalue)) (`KismetMathLibrary.Conv_DoubleToVector` (/ (`local.local_icon`) 2.0))) (`local.local_size`) (`local.local_offset`) (`local.local_zoom`) (/ (`local.local_icon`) 2.0)))
  (return _clamped_value _unclamped_value))

(fn `convert_world_to_exponent`
  (params (world_loc :type "Vector Structure"))
  (returns (map_location :type "Vector Structure"))
  (locals (local_input_loc :type "Vector Structure"))
  ;[1 1 1] Convert input location to map location.
  (set `local.local_input_loc` world_loc)
  (return (`KismetMathLibrary.GreaterGreater_VectorRotator` (`KismetMathLibrary.MakeVector` (`KismetMathLibrary.MapRangeUnclamped` (.x (`local.local_input_loc`)) (.x (`KismetMathLibrary.MakeVector` (- (.x (`self.map_origin`)) (/ (.x (`self.map_bounds`)) 2.0)) (- (.y (`self.map_origin`)) (/ (.y (`self.map_bounds`)) 2.0)) (- (.z (`self.map_origin`)) (/ (.z (`self.map_bounds`)) 2.0)))) (.x (`KismetMathLibrary.MakeVector` (+ (.x (`self.map_origin`)) (/ (.x (`self.map_bounds`)) 2.0)) (+ (.y (`self.map_origin`)) (/ (.y (`self.map_bounds`)) 2.0)) (+ (.z (`self.map_origin`)) (/ (.z (`self.map_bounds`)) 2.0)))) 1.0 -1.0) (`KismetMathLibrary.MapRangeUnclamped` (.y (`local.local_input_loc`)) (.y (`KismetMathLibrary.MakeVector` (- (.x (`self.map_origin`)) (/ (.x (`self.map_bounds`)) 2.0)) (- (.y (`self.map_origin`)) (/ (.y (`self.map_bounds`)) 2.0)) (- (.z (`self.map_origin`)) (/ (.z (`self.map_bounds`)) 2.0)))) (.y (`KismetMathLibrary.MakeVector` (+ (.x (`self.map_origin`)) (/ (.x (`self.map_bounds`)) 2.0)) (+ (.y (`self.map_origin`)) (/ (.y (`self.map_bounds`)) 2.0)) (+ (.z (`self.map_origin`)) (/ (.z (`self.map_bounds`)) 2.0)))) -1.0 1.0) (`KismetMathLibrary.MapRangeUnclamped` (.z (`local.local_input_loc`)) (.z (`KismetMathLibrary.MakeVector` (- (.x (`self.map_origin`)) (/ (.x (`self.map_bounds`)) 2.0)) (- (.y (`self.map_origin`)) (/ (.y (`self.map_bounds`)) 2.0)) (- (.z (`self.map_origin`)) (/ (.z (`self.map_bounds`)) 2.0)))) (.z (`KismetMathLibrary.MakeVector` (+ (.x (`self.map_origin`)) (/ (.x (`self.map_bounds`)) 2.0)) (+ (.y (`self.map_origin`)) (/ (.y (`self.map_bounds`)) 2.0)) (+ (.z (`self.map_origin`)) (/ (.z (`self.map_bounds`)) 2.0)))) -1.0 1.0)) (`KismetMathLibrary.MakeRotator` 0.0 0.0 (`self.capture_yaw`)))))

(fn `init_map`
  (params (map_id :type Name))
  (bind _returnvalue (`KismetArrayLibrary.Array_Find` (`self.Tags`) (`self.map_id`)))
  ;[1 1 1] Init map logic.
  (`|ExecutionSequence`
    (:`then_0`
      (if (>= _returnvalue 0)
        (`KismetArrayLibrary.Array_Remove` (`self.Tags`) _returnvalue)))
    (:`then_1`
      (set `self.map_id` map_id)
      (`KismetArrayLibrary.Array_AddUnique` (`self.Tags`) (`self.map_id`)))))

(fn `refresh_values`
  ;[1 1 1] Refresh minimap values.
  (`|ExecutionSequence`
    (:`then_0`
      (`SceneComponent.K2_SetRelativeLocation` (`self.map_capture`) (`KismetMathLibrary.MakeVector` 0.0 0.0 (`self.capture_height`)) false false)
      (`SceneComponent.K2_SetRelativeRotation` (`self.map_capture`) (`KismetMathLibrary.MakeRotator` 0.0 (* (`self.capture_angle`) -1.0) (`self.capture_yaw`)) false false))
    (:`then_1`
      (set `SceneCaptureComponent2D.ProjectionType` (`self.capture_type`) (`self.map_capture`))
      (set `SceneCaptureComponent2D.OrthoWidth` (`KismetMathLibrary.FMax` (.x (`self.map_bounds`)) (.y (`self.map_bounds`))) (`self.map_capture`))
      (set `SceneCaptureComponent2D.FOVAngle` (`self.capture_fov`) (`self.map_capture`))
      (`CameraComponent.SetProjectionMode` (`self.dummy_camera`) (`self.capture_type`))
      (`CameraComponent.SetOrthoWidth` (`self.dummy_camera`) (`KismetMathLibrary.FMax` (.x (`self.map_bounds`)) (.y (`self.map_bounds`))))
      (`CameraComponent.SetFieldOfView` (`self.dummy_camera`) (`self.capture_fov`))
      (`SceneComponent.K2_SetRelativeRotation` (`self.dummy_capture_region`) (`KismetMathLibrary.MakeRotator` 0.0 0.0 (`self.capture_yaw`)) false false)
      (`BoxComponent.SetBoxExtent` (`self.dummy_capture_region`) (/ (`self.map_bounds`) 2.0) false)
      (`SceneComponent.SetWorldScale3D` (`self.dummy_capture_zone`) (/ (`self.map_bounds`) 100.0)))
    (:`then_2`
      (set `SceneCaptureComponent2D.TextureTarget` (`self.texture_render`) (`self.map_capture`)))))

(fn `register_icon`
  (params (register_actor :type "Actor Object Reference") (icon_component :type "/Game/DLG_Tree/dmap_system/blueprints/bp_dlg_map_component Object Reference") (remove_icon :type Boolean))
  (locals (local_actor :type "Actor Object Reference") (local_remove :type Boolean) (local_component :type "/Game/DLG_Tree/dmap_system/blueprints/bp_dlg_map_component Object Reference"))
  ;[1 1 1] Register icons to track.
  (set `local.local_actor` register_actor)
  (set `local.local_component` icon_component)
  (set `local.local_remove` remove_icon)
  (`/Game/EditorBlueprintResources/StandardMacros.IsValid` (`self.w_target_map`)
    (:`Is Valid`
      (`/Game/DLG_Tree/dmap_system/widgets/w_02_map_image.add_icon` (`self.w_target_map`) (`local.local_actor`) (`local.local_component`) (`local.local_remove`)))))

(fn `set_map`
  (params (is_active :type Boolean) (map_widget :type "/Game/DLG_Tree/dmap_system/widgets/w_02_map_image Object Reference"))
  (bind _returnvalue (`KismetArrayLibrary.Array_Find` (`self.Tags`) "dlg_map_active"))
  ;[1 1 1] Set this map as active.
  (set `self.is_active` is_active)
  (set `self.w_target_map` map_widget)
  (if (`local.is_active`)
    (`KismetArrayLibrary.Array_AddUnique` (`self.Tags`) "dlg_map_active")
    (`/Game/EditorBlueprintResources/StandardMacros.IsValid` (`self.w_target_map`)
      (:`Is Valid`
        (`/Game/DLG_Tree/dmap_system/widgets/w_02_map_image.set_map` (`self.w_target_map`) self)))
    (elif (>= _returnvalue 0)
      (`KismetArrayLibrary.Array_Remove` (`self.Tags`) _returnvalue))))

(fn `set_origin`
  (params (map_origin :type "Vector Structure") (map_bounds :type "Vector Structure"))
  ;[1 1 1] Set origin for map bounds.
  (set `self.map_origin` map_origin)
  (set `self.map_bounds` map_bounds)
  (`self.K2_SetActorLocation` (`self.map_origin`))
  (`self.refresh_values`))

(fn `UserConstructionScript`
  ;[1 1 1] Refresh initial capture values.
  (`self.refresh_values`))