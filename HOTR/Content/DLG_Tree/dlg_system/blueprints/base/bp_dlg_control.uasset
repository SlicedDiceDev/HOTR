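; Input relay actor for the dialogue system, used to skip lines and select choices in running dialogues, not to start them.
; Gamepad action, mouse and number key events become named IDs with pressed state in DlgAction.
; It gathers active Bp_dlg_actors, sorts them nearest first, filters by conflict priority and block/ignore lists, then calls DlgControlsAction on those passing.
; Stick and trigger axes route to DlgAxis, which is an empty stub.
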(event `InputAction|q_special_l` :consume false :paused true :overrideparent false
  (params (Key :type "Key Structure"))
  ;[0.3694 0.7653 1] Special L/R.
  (:`Pressed`
    (`self.dlg_action` Key "special_l" :!label _label))
  (:`Released`
    (goto _label)))

(event `InputAction|q_shoulder_l` :consume false :paused true :overrideparent false
  (params (Key :type "Key Structure"))
  ;[0.3694 0.7653 1] Shoulder L/R.
  (:`Pressed`
    (`self.dlg_action` Key "shoulder_l" :!label _label_2))
  (:`Released`
    (goto _label_2)))

(event `InputAction|q_trigger_l` :consume false :paused true :overrideparent false
  (params (Key :type "Key Structure"))
  ;[0.3694 0.7653 1] Button Trigger L/R.
  (:`Pressed`
    (`self.dlg_action` Key "trigger_l" :!label _label_3))
  (:`Released`
    (goto _label_3)))

(event `InputAction|q_dpad_u` :consume false :paused true :overrideparent false
  (params (Key :type "Key Structure"))
  ;[0.3694 0.7653 1] Dpad U/D.
  (:`Pressed`
    (`self.dlg_action` Key "dpad_u" :!label _label_4))
  (:`Released`
    (goto _label_4)))

(event `InputAction|q_dpad_l` :consume false :paused true :overrideparent false
  (params (Key :type "Key Structure"))
  ;[0.3694 0.7653 1] Dpad L/R.
  (:`Pressed`
    (`self.dlg_action` Key "dpad_l" :!label _label_5))
  (:`Released`
    (goto _label_5)))

(event `self.ReceiveBeginPlay`
  ;[1 1 1] Beginplay is here.
  (`self.EnableInput` (`GameplayStatics.GetPlayerController` 0)))

(event `InputAction|q_special_r` :consume false :paused true :overrideparent false
  (params (Key :type "Key Structure"))
  ;[0.3694 0.7653 1] Special L/R.
  (:`Pressed`
    (`self.dlg_action` Key "special_r" :!label _label_6))
  (:`Released`
    (goto _label_6)))

(event `InputAction|q_shoulder_r` :consume false :paused true :overrideparent false
  (params (Key :type "Key Structure"))
  ;[0.3694 0.7653 1] Shoulder L/R.
  (:`Pressed`
    (`self.dlg_action` Key "shoulder_r" :!label _label_7))
  (:`Released`
    (goto _label_7)))

(event `InputAction|q_trigger_r` :consume false :paused true :overrideparent false
  (params (Key :type "Key Structure"))
  ;[0.3694 0.7653 1] Button Trigger L/R.
  (:`Pressed`
    (`self.dlg_action` Key "trigger_r" :!label _label_8))
  (:`Released`
    (goto _label_8)))

(event `InputAction|q_dpad_d` :consume false :paused true :overrideparent false
  (params (Key :type "Key Structure"))
  ;[0.3694 0.7653 1] Dpad U/D.
  (:`Pressed`
    (`self.dlg_action` Key "dpad_d" :!label _label_9))
  (:`Released`
    (goto _label_9)))

(event `InputAction|q_dpad_r` :consume false :paused true :overrideparent false
  (params (Key :type "Key Structure"))
  ;[0.3694 0.7653 1] Dpad L/R.
  (:`Pressed`
    (`self.dlg_action` Key "dpad_r" :!label _label_10))
  (:`Released`
    (goto _label_10)))

(event `InputAction|q_thumb_l` :consume false :paused true :overrideparent false
  (params (Key :type "Key Structure"))
  ;[0.3694 0.7653 1] Thumb L/R.
  (:`Pressed`
    (`self.dlg_action` Key "thumb_l" :!label _label_11))
  (:`Released`
    (goto _label_11)))

(event `InputAction|q_face_u` :consume false :paused true :overrideparent false
  (params (Key :type "Key Structure"))
  ;[0.3694 0.7653 1] Face U/D.
  (:`Pressed`
    (`self.dlg_action` Key "face_u" :!label _label_12))
  (:`Released`
    (goto _label_12)))

(event `InputAction|q_face_l` :consume false :paused true :overrideparent false
  (params (Key :type "Key Structure"))
  ;[0.3694 0.7653 1] Face L/R.
  (:`Pressed`
    (`self.dlg_action` Key "face_l" :!label _label_13))
  (:`Released`
    (goto _label_13)))

(event `Key|LeftMouseButton` :consume false :paused true :overrideparent false
  (params (Key :type "Key Structure"))
  ;[0.3694 1 0.3694] Mouse Input.
  (:`Pressed`
    (`self.dlg_action` Key "mouse_l" :!label _label_14))
  (:`Released`
    (goto _label_14)))

(event `Key|One` :consume false :paused true :overrideparent false
  (params (Key :type "Key Structure"))
  ;[1 1 1] Numeric selection for DLG.
  ; PC keyboard controls.
  (:`Pressed`
    (`self.dlg_action` Key "1" :!label _label_15))
  (:`Released`
    (goto _label_15)))

(event `Key|Six` :consume false :paused true :overrideparent false
  (params (Key :type "Key Structure"))
  ;[1 1 1] Numeric selection for DLG.
  ; PC keyboard controls.
  (:`Pressed`
    (`self.dlg_action` Key "6" :!label _label_16))
  (:`Released`
    (goto _label_16)))

(event `Key|RightMouseButton` :consume false :paused true :overrideparent false
  (params (Key :type "Key Structure"))
  ;[0.3694 1 0.3694] Mouse Input.
  (:`Pressed`
    (`self.dlg_action` Key "mouse_r" :!label _label_17))
  (:`Released`
    (goto _label_17)))

(event `InputAction|q_thumb_r` :consume false :paused true :overrideparent false
  (params (Key :type "Key Structure"))
  ;[0.3694 0.7653 1] Thumb L/R.
  (:`Pressed`
    (`self.dlg_action` Key "thumb_r" :!label _label_18))
  (:`Released`
    (goto _label_18)))

(event `InputAction|q_face_d` :consume false :paused true :overrideparent false
  (params (Key :type "Key Structure"))
  ;[0.3694 0.7653 1] Face U/D.
  (:`Pressed`
    (`self.dlg_action` Key "face_d" :!label _label_19))
  (:`Released`
    (goto _label_19)))

(event `InputAction|q_face_r` :consume false :paused true :overrideparent false
  (params (Key :type "Key Structure"))
  ;[0.3694 0.7653 1] Face L/R.
  (:`Pressed`
    (`self.dlg_action` Key "face_r" :!label _label_20))
  (:`Released`
    (goto _label_20)))

(event `Key|Two` :consume false :paused true :overrideparent false
  (params (Key :type "Key Structure"))
  ;[1 1 1] Numeric selection for DLG.
  ; PC keyboard controls.
  (:`Pressed`
    (`self.dlg_action` Key "2" :!label _label_21))
  (:`Released`
    (goto _label_21)))

(event `Key|Seven` :consume false :paused true :overrideparent false
  (params (Key :type "Key Structure"))
  ;[1 1 1] Numeric selection for DLG.
  ; PC keyboard controls.
  (:`Pressed`
    (`self.dlg_action` Key "7" :!label _label_22))
  (:`Released`
    (goto _label_22)))

(event `Key|MiddleMouseButton` :consume false :paused true :overrideparent false
  (params (Key :type "Key Structure"))
  ;[0.3694 1 0.3694] Mouse Input.
  (:`Pressed`
    (`self.dlg_action` Key "mouse_m" :!label _label_23))
  (:`Released`
    (goto _label_23)))

(event `Key|Three` :consume false :paused true :overrideparent false
  (params (Key :type "Key Structure"))
  ;[1 1 1] Numeric selection for DLG.
  ; PC keyboard controls.
  (:`Pressed`
    (`self.dlg_action` Key "3" :!label _label_24))
  (:`Released`
    (goto _label_24)))

(event `Key|Eight` :consume false :paused true :overrideparent false
  (params (Key :type "Key Structure"))
  ;[1 1 1] Numeric selection for DLG.
  ; PC keyboard controls.
  (:`Pressed`
    (`self.dlg_action` Key "8" :!label _label_25))
  (:`Released`
    (goto _label_25)))

(event `Key|Four` :consume false :paused true :overrideparent false
  (params (Key :type "Key Structure"))
  ;[1 1 1] Numeric selection for DLG.
  ; PC keyboard controls.
  (:`Pressed`
    (`self.dlg_action` Key "4" :!label _label_26))
  (:`Released`
    (goto _label_26)))

(event `Key|Nine` :consume false :paused true :overrideparent false
  (params (Key :type "Key Structure"))
  ;[1 1 1] Numeric selection for DLG.
  ; PC keyboard controls.
  (:`Pressed`
    (`self.dlg_action` Key "9" :!label _label_27))
  (:`Released`
    (goto _label_27)))

(event `Key|Five` :consume false :paused true :overrideparent false
  (params (Key :type "Key Structure"))
  ;[1 1 1] Numeric selection for DLG.
  ; PC keyboard controls.
  (:`Pressed`
    (`self.dlg_action` Key "5" :!label _label_28))
  (:`Released`
    (goto _label_28)))

(event `Key|Zero` :consume false :paused true :overrideparent false
  (params (Key :type "Key Structure"))
  ;[1 1 1] Numeric selection for DLG.
  ; PC keyboard controls.
  (:`Pressed`
    (`self.dlg_action` Key "10" :!label _label_29))
  (:`Released`
    (goto _label_29)))

(event `InputAxis|q_move_x` :consume false :paused true :overrideparent false
  (params (AxisValue :type "Float (single-precision)"))
  ;[0.5249 0.5873 1] Axis Sticks L/R -- Axis Triggers L/R.
  (`self.dlg_axis` "stick_l" AxisValue (stale `InputAxis|q_move_y` AxisValue) :!label _label_30))

(event `InputAxis|q_turn_x` :consume false :paused true :overrideparent false
  (params (AxisValue :type "Float (single-precision)"))
  ;[0.5249 0.5873 1] Axis Sticks L/R -- Axis Triggers L/R.
  (`self.dlg_axis` "stick_r" AxisValue (* (stale `InputAxis|q_turn_y` AxisValue) -1.0) :!label _label_31))

(event `InputAxis|q_trigger_axis_l` :consume false :paused true :overrideparent false
  (params (AxisValue :type "Float (single-precision)"))
  ;[0.5249 0.5873 1] Axis Sticks L/R -- Axis Triggers L/R.
  (`self.dlg_axis` "trigger_axis_l" AxisValue AxisValue))

(event `InputAxis|q_move_y` :consume false :paused true :overrideparent false
  (params (AxisValue :type "Float (single-precision)"))
  ;[0.5249 0.5873 1] Axis Sticks L/R -- Axis Triggers L/R.
  (goto _label_30))

(event `InputAxis|q_turn_y` :consume false :paused true :overrideparent false
  (params (AxisValue :type "Float (single-precision)"))
  ;[0.5249 0.5873 1] Axis Sticks L/R -- Axis Triggers L/R.
  (goto _label_31))

(event `InputAxis|q_trigger_axis_r` :consume false :paused true :overrideparent false
  (params (AxisValue :type "Float (single-precision)"))
  ;[0.5249 0.5873 1] Axis Sticks L/R -- Axis Triggers L/R.
  (`self.dlg_axis` "trigger_axis_r" AxisValue AxisValue))

(fn `dlg_action`
  (params (input_key :type "Key Structure") (input_id :type Name))
  (locals (local_key :type "Key Structure") (local_pressed :type Boolean) (local_input :type Name) (local_ignore :type "Array of Name") (local_block :type "Array of Name") (local_sorted_list :type "Array of /Game/DLG_Tree/dlg_system/blueprints/base/bp_dlg_actor Object Reference") (local_unblocked_list :type "Array of /Game/DLG_Tree/dlg_system/blueprints/base/bp_dlg_actor Object Reference"))
  ;[1 1 1] Action input convert func.
  (set `local.local_key` input_key)
  (set `local.local_input` input_id)
  (set `local.local_pressed` (`PlayerController.IsInputKeyDown` (`GameplayStatics.GetPlayerController` 0) (`local.local_key`)))
  (bind _sorted_actors_reversed (`self.sort_dlg_actors`))
  (set `local.local_sorted_list` _sorted_actors_reversed)
  (if (`KismetArrayLibrary.Array_IsValidIndex` (`local.local_sorted_list`))
    (`|ExecutionSequence`
      (:`then_0`
        (if (<= (`KismetArrayLibrary.Array_Length` (`local.local_sorted_list`)) 1)
          (`KismetArrayLibrary.Array_Add` (`local.local_unblocked_list`) (`|GetArrayItem` (`local.local_sorted_list`)))
          (else
            (bind (_array_element _array_index) (`/Game/EditorBlueprintResources/StandardMacros.ForEachLoop` (`local.local_sorted_list`))
              (:`LoopBody`
                (bind (_array_element_2 _array_index_2) (`/Game/EditorBlueprintResources/StandardMacros.ForEachLoop` (`local.local_sorted_list`))
                  (:`LoopBody`
                    (if (!= _array_index_2 _array_index)
                      (bind (_conflict_priority _ignore_data _block_data) (break `/Game/DLG_Tree/dlg_system/structs/04_data/s_dlg_conflicts` (`/Game/DLG_Tree/dlg_system/blueprints/base/bp_dlg_actor.dlg_conflict_data` _array_element_2)))
                      (bind (_conflict_priority_2 _ignore_data_2) (break `/Game/DLG_Tree/dlg_system/structs/04_data/s_dlg_conflicts` (`/Game/DLG_Tree/dlg_system/blueprints/base/bp_dlg_actor.dlg_conflict_data` _array_element)))
                      (if (> _conflict_priority _conflict_priority_2)
                        _
                        (elif (or (`KismetArrayLibrary.Array_Contains` _block_data (`/Game/DLG_Tree/dlg_system/blueprints/base/bp_dlg_actor.dlg_unique_id` _array_element)) (`KismetArrayLibrary.Array_Contains` _block_data "any"))
                          _
                          (elif (not (or (`KismetArrayLibrary.Array_Contains` _ignore_data_2 (`/Game/DLG_Tree/dlg_system/blueprints/base/bp_dlg_actor.dlg_unique_id` _array_element_2)) (`KismetArrayLibrary.Array_Contains` _ignore_data_2 "any")))
                            (`KismetArrayLibrary.Array_Add` (`local.local_unblocked_list`) _array_element))))))))))))
      (:`then_1`
        (bind _array_element_3 (`/Game/EditorBlueprintResources/StandardMacros.ForEachLoop` (`local.local_unblocked_list`))
          (:`LoopBody`
            (`/Game/DLG_Tree/dlg_system/blueprints/base/bp_dlg_actor.dlg_controls_action` _array_element_3 (`local.local_input`) (`local.local_pressed`))))))))

(fn `dlg_axis`
  (params (input_id :type Name) (axis_x :type "Float (double-precision)") (axis_y :type "Float (double-precision)"))
  (locals (local_ignore :type "Array of Name") (local_block :type "Array of Name") (local_input :type Name))
  ;[1 1 1] Axis input convert func,
  ; not implemented.
)

(fn `sort_dlg_actors`
  (returns (sorted_actors_reversed :type "Array of /Game/DLG_Tree/dlg_system/blueprints/base/bp_dlg_actor Object Reference"))
  (locals (local_actors_distance :type "Array of Float (double-precision)") (local_actors_list :type "Array of /Game/DLG_Tree/dlg_system/blueprints/base/bp_dlg_actor Object Reference") (local_sorted_actors :type "Array of /Game/DLG_Tree/dlg_system/blueprints/base/bp_dlg_actor Object Reference") (local_min_index :type Integer :default 0))
  ;[1 1 1] Clean sorting logic, finds all DLG actors existing in the world, and sorting them by distance.
  ; This is to proceed input in distance priority, keep in mind this input actor is not for starting dialogues,
  ; this is used to call skip function and select choices, so if there is multiple dynamic dialogues, skipped will be closest one.
  ;
  ; Keep in mind if there is very-very large DLG actors in the world then other sorting logic should be used instead of this one,
  ; method like sphere tracing from player location and etc to find nearby dialogues,
  ; but yet this method works fine for fine large amount of dialogues.
  (bind _outactors (`GameplayStatics.GetAllActorsOfClass` "/Game/DLG_Tree/dlg_system/blueprints/base/bp_dlg_actor.bp_dlg_actor_C"))
  (bind _array_element (`/Game/EditorBlueprintResources/StandardMacros.ForEachLoop` _outactors)
    (:`LoopBody`
      (if (`/Game/DLG_Tree/dlg_system/blueprints/base/bp_dlg_actor.is_dlg_active` _array_element)
        (`KismetArrayLibrary.Array_Add` (`local.local_actors_distance`) (`self.GetDistanceTo` _array_element (`GameplayStatics.GetPlayerPawn` 0)))
        (`KismetArrayLibrary.Array_Add` (`local.local_actors_list`) _array_element)))
    (:`Completed`
      (set `local.local_min_index` (`KismetMathLibrary.MinOfFloatArray` (`local.local_actors_distance`)) :!label _label)
      (if (>= (`local.local_min_index`) 0)
        (`KismetArrayLibrary.Array_Add` (`local.local_sorted_actors`) (`|GetArrayItem` (`local.local_actors_list`) (`local.local_min_index`)))
        (`KismetArrayLibrary.Array_Remove` (`local.local_actors_distance`) (`local.local_min_index`))
        (`KismetArrayLibrary.Array_Remove` (`local.local_actors_list`) (`local.local_min_index`))
        (goto _label)
        (else
          (return (`local.local_sorted_actors`)))))))

(fn `UserConstructionScript`)