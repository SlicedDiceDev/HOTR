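; Blueprint function library for the DLG dialogue and quest system, providing component lookups and quick condition checks.
; Getters fetch dialogue, quest and map components from an actor, and the notification component from the first player controller, each with a validity flag.
; Condition converters resolve actors by ID, then test stored NPC replies and choices or player quest, objective and sub-objective status.
; The base converter ANDs both results; empty lists pass.
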(fn `dlg_convert_base_condition`
  (params (dlg_quick_condition :type "/Game/DLG_Tree/dlg_system/structs/04_data/s_dlg_quick_condition_base Structure"))
  (returns (return_condition :type Boolean))
  (bind (_dlg_conditions _quest_conditions) (break `/Game/DLG_Tree/dlg_system/structs/04_data/s_dlg_quick_condition_base` dlg_quick_condition))
  ;[1 1 1] DLG convert quick DLG conditions for various checks.
  (return (and (`self.dlg_convert_dlg_condition` null _dlg_conditions) (`self.dlg_convert_quest_condition` _quest_conditions))))

(fn `dlg_convert_dlg_condition`
  (params (dlg_conditions :type "Array of /Game/DLG_Tree/dlg_system/structs/04_data/s_dlg_quick_condition_dlg Structure"))
  (returns (return_condition :type Boolean))
  (locals (local_dlg :type "/Game/DLG_Tree/dlg_system/blueprints/base/bp_dlg_actor Object Reference") (local_condition_true :type Boolean :default false))
  ;[1 1 1] DLG convert quick DLG conditions for various checks.
  (if (not (`KismetArrayLibrary.Array_IsValidIndex` dlg_conditions))
    (set `local.local_condition_true` true))
  (bind _array_element (`/Game/EditorBlueprintResources/StandardMacros.ForEachLoopWithBreak` dlg_conditions :!label _label)
    (:`LoopBody`
      (`|ExecutionSequence`
        (:`then_0`
          (bind (_npc_base_id _dlg_unique_id _dlg_branch_id _dlg_reply_id _dlg_choice_id _reply_true _choice_true) (break `/Game/DLG_Tree/dlg_system/structs/04_data/s_dlg_quick_condition_dlg` _array_element))
          (bind (_is_valid _actor_reference) (`/Game/MSL_Toolkit/initial_system/msl_function_library.msl_get_actor_by_id` _npc_base_id))
          (if _is_valid
            (bind (_is_valid_2 _dlg_reference) (`self.dlg_get_dlg_component` _actor_reference))
            (if _is_valid_2
              (bind (_is_valid_3 _found_index _dlg_actor) (`/Game/DLG_Tree/dlg_system/blueprints/base/bp_dlg_component.get_dlg` _dlg_reference _dlg_unique_id))
              (set `local.local_dlg` _dlg_actor))))
        (:`then_1`
          (`/Game/EditorBlueprintResources/StandardMacros.IsValid` (`local.local_dlg`)
            (:`Is Valid`
              (`|ExecutionSequence`
                (:`then_0`
                  (if (!= _dlg_reply_id "None")
                    (bind _returnvalue (== _dlg_branch_id "None"))
                    (bind _is_valid_4 (`/Game/DLG_Tree/dlg_system/blueprints/base/bp_dlg_actor.get_storage_reply` (`local.local_dlg`) _returnvalue _dlg_branch_id _dlg_reply_id))
                    (set `local.local_condition_true` (== _is_valid_4 _reply_true))))
                (:`then_1`
                  (if (!= _dlg_choice_id "None")
                    (bind _is_valid_5 (`/Game/DLG_Tree/dlg_system/blueprints/base/bp_dlg_actor.get_storage_choice` (`local.local_dlg`) _returnvalue _dlg_branch_id _dlg_choice_id))
                    (set `local.local_condition_true` (== _is_valid_5 _choice_true))))
                (:`then_2`
                  (if (not (`local.local_condition_true`))
                    (goto _label :!via `Break`)))))))))
    (:`Completed`
      (return (`local.local_condition_true`)))))

(fn `dlg_convert_quest_condition`
  (params (quest_conditions :type "Array of /Game/DLG_Tree/dlg_system/structs/04_data/s_dlg_quick_condition_quest Structure"))
  (returns (return_condition :type Boolean))
  (locals (local_quest :type "/Game/DLG_Tree/dqst_system/blueprints/bp_quest_actor Object Reference") (local_condition_true :type Boolean :default false))
  (bind (_is_valid _actor_reference) (`/Game/MSL_Toolkit/initial_system/msl_function_library.msl_get_actor_by_id` "player"))
  (bind (_is_valid_2 _quest_reference) (`self.dlg_get_quest_component` _actor_reference))
  (bind _quest_status (`/Game/DLG_Tree/dqst_system/blueprints/bp_quest_actor.quest_status` (`local.local_quest`)))
  (bind _returnvalue (`|EnumEquality` _quest_status "NewEnumerator0"))
  (bind _returnvalue_2 (`|EnumEquality` _quest_status "NewEnumerator3"))
  ;[1 1 1] DLG convert quick DLG conditions for various checks.
  (if (not (`KismetArrayLibrary.Array_IsValidIndex` quest_conditions))
    (set `local.local_condition_true` true))
  (bind _array_element (`/Game/EditorBlueprintResources/StandardMacros.ForEachLoopWithBreak` quest_conditions :!label _label)
    (:`LoopBody`
      (`|ExecutionSequence`
        (:`then_0`
          (if _is_valid
            (if _is_valid_2
              (bind (_quest_id _objective_id _sub_objective_id _quest_true _objective_true _sub_objective_true) (break `/Game/DLG_Tree/dlg_system/structs/04_data/s_dlg_quick_condition_quest` _array_element))
              (bind (_is_valid_3 _found_index _quest_actor) (`/Game/DLG_Tree/dqst_system/blueprints/bp_quest_component.get_quest` _quest_reference _quest_id))
              (set `local.local_quest` _quest_actor))))
        (:`then_1`
          (`/Game/EditorBlueprintResources/StandardMacros.IsValid` (`local.local_quest`)
            (:`Is Valid`
              (`|ExecutionSequence`
                (:`then_0`
                  (switch `/Game/DLG_Tree/dqst_system/structs/09_enums/enum_quest_phase` _quest_true
                    (:`NewEnumerator0`
                      (set `local.local_condition_true` (`|EnumEquality` _quest_status "NewEnumerator2")))
                    (:`NewEnumerator1`
                      (set `local.local_condition_true` _returnvalue))
                    (:`NewEnumerator2`
                      (set `local.local_condition_true` _returnvalue_2))
                    (:`NewEnumerator3`
                      (set `local.local_condition_true` (or _returnvalue _returnvalue_2)))))
                (:`then_1`
                  (if (!= _objective_id "None")
                    (bind (_objective_exist _objective_is_current _objective_index _objective_data) (`/Game/DLG_Tree/dqst_system/blueprints/bp_quest_actor.get_objective` (`local.local_quest`) _objective_id "None" false))
                    (if _objective_exist
                      (switch `/Game/DLG_Tree/dqst_system/structs/09_enums/enum_quest_phase` _objective_true
                        (:`NewEnumerator0`
                          (bind (_objective_id_2 _objective_result) (break `/Game/DLG_Tree/dqst_system/structs/02_objective/s_quest_objective_dynamic` (`.objective_dynamic_36_2E72E27A43E1FD7F6C35A480D967F653` (break `/Game/DLG_Tree/dqst_system/structs/02_objective/s_quest_objective_data` _objective_data))))
                          (set `local.local_condition_true` (`|EnumEquality` _objective_result "NewEnumerator2")))
                        (:`NewEnumerator1`
                          (bind _returnvalue_3 (`|EnumEquality` _objective_result "NewEnumerator0"))
                          (set `local.local_condition_true` _returnvalue_3))
                        (:`NewEnumerator2`
                          (bind _returnvalue_4 (`|EnumEquality` _objective_result "NewEnumerator3"))
                          (set `local.local_condition_true` _returnvalue_4))
                        (:`NewEnumerator3`
                          (set `local.local_condition_true` (or _returnvalue_3 _returnvalue_4)))))))
                (:`then_2`
                  (if (!= _sub_objective_id "None")
                    (bind (_objective_exist_2 _objective_is_current_2 _objective_index_2 _objective_data_2 _sub_objective_exist _sub_objective_index _sub_objective_data) (`/Game/DLG_Tree/dqst_system/blueprints/bp_quest_actor.get_objective` (`local.local_quest`) _objective_id _sub_objective_id false))
                    (if _sub_objective_exist
                      (switch `/Game/DLG_Tree/dqst_system/structs/09_enums/enum_quest_phase` _sub_objective_true
                        (:`NewEnumerator0`
                          (bind (_sub_objective_id_2 _current_progress _objective_status) (break `/Game/DLG_Tree/dqst_system/structs/03_sub_objective/s_quest_sub_objective_dynamic` (`.sub_objective_dynamic_16_44509D1B4E07798A74E7FCAAFEEF1857` (break `/Game/DLG_Tree/dqst_system/structs/03_sub_objective/s_quest_sub_objective_data` _sub_objective_data))))
                          (set `local.local_condition_true` (`|EnumEquality` _objective_status "NewEnumerator2")))
                        (:`NewEnumerator1`
                          (bind _returnvalue_5 (`|EnumEquality` _objective_status "NewEnumerator0"))
                          (set `local.local_condition_true` _returnvalue_5))
                        (:`NewEnumerator2`
                          (bind _returnvalue_6 (`|EnumEquality` _objective_status "NewEnumerator3"))
                          (set `local.local_condition_true` _returnvalue_6))
                        (:`NewEnumerator3`
                          (set `local.local_condition_true` (or _returnvalue_5 _returnvalue_6)))))))
                (:`then_3`
                  (if (not (`local.local_condition_true`))
                    (goto _label :!via `Break`)))))))))
    (:`Completed`
      (return (`local.local_condition_true`)))))

(fn `dlg_get_dlg_component`
  (params (target_actor :type "Actor Object Reference"))
  (returns (is_valid :type Boolean) (dlg_reference :type "/Game/DLG_Tree/dlg_system/blueprints/base/bp_dlg_component Object Reference"))
  (bind _returnvalue (`Actor.GetComponentByClass` target_actor "/Game/DLG_Tree/dlg_system/blueprints/base/bp_dlg_component.bp_dlg_component_C"))
  ;[1 1 1] Get dlg component of actor.
  (`/Game/EditorBlueprintResources/StandardMacros.IsValid` target_actor
    (:`Is Valid`
      (`/Game/EditorBlueprintResources/StandardMacros.IsValid` _returnvalue
        (:`Is Valid`
          (return true _returnvalue))
        (:`Is Not Valid`
          _)))
    (:`Is Not Valid`
      _))
  (return false null))

(fn `dlg_get_map_component`
  (params (target_actor :type "Actor Object Reference"))
  (returns (is_valid :type Boolean) (map_reference :type "/Game/DLG_Tree/dmap_system/blueprints/bp_dlg_map_component Object Reference"))
  (bind _returnvalue (`Actor.GetComponentByClass` target_actor "/Game/DLG_Tree/dmap_system/blueprints/bp_dlg_map_component.bp_dlg_map_component_C"))
  ;[1 1 1] Get map component of actor.
  (`/Game/EditorBlueprintResources/StandardMacros.IsValid` target_actor
    (:`Is Valid`
      (`/Game/EditorBlueprintResources/StandardMacros.IsValid` _returnvalue
        (:`Is Valid`
          (return true _returnvalue))
        (:`Is Not Valid`
          _)))
    (:`Is Not Valid`
      _))
  (return false null))

(fn `dlg_get_notification_component`
  (returns (is_valid :type Boolean) (notification_reference :type "/Game/DLG_Tree/dqst_system/blueprints/bp_notification_component Object Reference"))
  (bind _returnvalue (`GameplayStatics.GetPlayerController` null))
  (bind _returnvalue_2 (`Actor.GetComponentByClass` _returnvalue "/Game/DLG_Tree/dqst_system/blueprints/bp_notification_component.bp_notification_component_C"))
  ;[1 1 1] Get map component of actor.
  (`/Game/EditorBlueprintResources/StandardMacros.IsValid` _returnvalue
    (:`Is Valid`
      (`/Game/EditorBlueprintResources/StandardMacros.IsValid` _returnvalue_2
        (:`Is Valid`
          (return true _returnvalue_2))
        (:`Is Not Valid`
          _)))
    (:`Is Not Valid`
      _))
  (return false _returnvalue_2))

(fn `dlg_get_quest_component`
  (params (target_actor :type "Actor Object Reference"))
  (returns (is_valid :type Boolean) (quest_reference :type "/Game/DLG_Tree/dqst_system/blueprints/bp_quest_component Object Reference"))
  (bind _returnvalue (`Actor.GetComponentByClass` target_actor "/Game/DLG_Tree/dqst_system/blueprints/bp_quest_component.bp_quest_component_C"))
  ;[1 1 1] Get qst component of actor.
  (`/Game/EditorBlueprintResources/StandardMacros.IsValid` target_actor
    (:`Is Valid`
      (`/Game/EditorBlueprintResources/StandardMacros.IsValid` _returnvalue
        (:`Is Valid`
          (return true _returnvalue))
        (:`Is Not Valid`
          _)))
    (:`Is Not Valid`
      _))
  (return false null))