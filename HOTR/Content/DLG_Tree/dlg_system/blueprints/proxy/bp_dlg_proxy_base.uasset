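; Base proxy actor for the dialogue system, linked to a dialogue actor and a proxy ID and hidden in game on init.
; Empty custom init and tick events act as hooks for child proxies.
; Float variables live in parallel ID and value arrays, with set adding missing IDs and get defaulting to zero.
; It also stores a skeletal mesh list and builds pose snapshots from a mesh's socket transforms in parent-bone space.
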(event `proxy_init`
  (params (dlg_actor :type "/Game/DLG_Tree/dlg_system/blueprints/base/bp_dlg_actor Object Reference") (proxy_id :type Name))
  ;[1 1 1] Proxy parent base actor,
  ; beginplay is here.
  (set `self.dlg_actor` dlg_actor)
  (set `self.proxy_id` proxy_id)
  (`|ExecutionSequence`
    (:`then_0`
      (`self.SetActorHiddenInGame` true))
    (:`then_1`
      (`self.custom_proxy_init`))))

(event `self.ReceiveTick`
  (params (DeltaSeconds :type "Float (single-precision)"))
  ;[1 1 1] Proxy parent base actor,
  ; beginplay is here.
  (`|ExecutionSequence`
    (:`then_1`
      (`self.custom_proxy_tick` DeltaSeconds))))

(event `custom_proxy_init`
  ;[1 1 1] Proxy parent base actor,
  ; beginplay is here.
)

(event `custom_proxy_tick`
  (params (delta_seconds :type "Float (double-precision)"))
  ;[1 1 1] Proxy parent base actor,
  ; beginplay is here.
)

(fn `find_var_id`
  (params (var_id :type Name))
  (returns (is_valid :type Boolean) (found_index :type Integer))
  (bind _returnvalue (`KismetArrayLibrary.Array_Find` (`self.var_id`) var_id))
  (bind _returnvalue_2 (>= _returnvalue 0))
  ;[1 1 1] Find Proxy var.
  (if _returnvalue_2
    (return _returnvalue_2 _returnvalue)
    (else
      (return false 0))))

(fn `get_float_var`
  (params (var_id :type Name))
  (returns (return_value :type "Float (double-precision)"))
  ;[1 1 1] Get variable logic.
  (bind (_is_valid _found_index) (`self.find_var_id` var_id))
  (if _is_valid
    (return (`|GetArrayItem` (`self.var_float`) _found_index))
    (else
      (return 0.0))))

(fn `set_float_var`
  (params (var_id :type Name) (var_value :type "Float (double-precision)"))
  (returns (return_value :type "Float (double-precision)"))
  (locals (local_id :type Name) (local_value :type "Float (double-precision)"))
  ;[1 1 1] Update variable logic.
  (set `local.local_id` var_id)
  (set `local.local_value` var_value)
  (`|ExecutionSequence`
    (:`then_0`
      (bind (_is_valid _found_index) (`self.find_var_id` (`local.local_id`)))
      (if _is_valid
        (`KismetArrayLibrary.Array_Set` (`self.var_float`) _found_index (`local.local_value`))
        (else
          (`KismetArrayLibrary.Array_Add` (`self.var_id`) (`local.local_id`))
          (`KismetArrayLibrary.Array_Add` (`self.var_float`) (`local.local_value`)))))
    (:`then_1`
      (return (`local.local_value`)))))

(fn `set_mesh_list`
  (params (mesh_list :type "Array of SkeletalMeshComponent Object Reference"))
  ;[1 1 1] Set skeletal mesh list.
  (set `self.mesh_list` mesh_list))

(fn `snapshot_mesh`
  (params (mesh_component :type "SkeletalMeshComponent Object Reference") (snapshot_name :type Name))
  (returns (snapshot_data :type "PoseSnapshot Structure"))
  (locals (local_mesh :type "SkeletalMeshComponent Object Reference") (local_name :type "Array of Name") (local_transform :type "Array of Transform Structure"))
  ;[1 1 1] Snapshot all bones of the input mesh, and return as snapshot data.
  (bind _output_get (set `local.local_mesh` mesh_component))
  (`/Game/EditorBlueprintResources/StandardMacros.IsValid` _output_get
    (:`Is Valid`
      (set `local.local_name` (`SceneComponent.GetAllSocketNames` (`local.local_mesh`)))
      (bind _array_element (`/Game/EditorBlueprintResources/StandardMacros.ForEachLoop` (`local.local_name`))
        (:`LoopBody`
          (`KismetArrayLibrary.Array_Add` (`local.local_transform`) (`SceneComponent.GetSocketTransform` (`local.local_mesh`) _array_element "RTS_ParentBoneSpace")))
        (:`Completed`
          (return (make `PoseSnapshot` (`local.local_transform`) (`local.local_name`) (`KismetStringLibrary.Conv_StringToName` (`KismetSystemLibrary.GetDisplayName` (`local.local_mesh`))) snapshot_name true)))))))

(fn `UserConstructionScript`)