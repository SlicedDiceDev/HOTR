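; Static camera rig actor attached to interlocutors while a DLG dialogue is active, providing their shots.
; On init it registers its camera components by object name in parallel ID and component lists.
; SetActiveCamera deactivates all registered cameras, then activates the requested one.
; GetAutoCam picks front, left or right face shots, randomly or opposite the last side shot when the interlocutor changes, keeping the 180-degree rule.
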(event `init_interlocutor`
  (params (interlocutor_id :type Name))
  ;[1 1 1] Beginplay is here,
  ; this is static actor cam, all DLG influenced actors
  ; will have this actor attached to them while DLG is active.
  (set `self.interlocutor_id` interlocutor_id)
  (bind _array_element (`/Game/EditorBlueprintResources/StandardMacros.ForEachLoop` (`self.K2_GetComponentsByClass` "/Script/Engine.CameraComponent"))
    (:`LoopBody`
      (`self.add_camera` (`KismetStringLibrary.Conv_StringToName` (`KismetSystemLibrary.GetObjectName` _array_element)) _array_element))))

(fn `add_camera`
  (params (camera_id :type Name) (camera_component :type "CameraComponent Object Reference"))
  ;[1 1 1] Add camera component to array list.
  (bind _is_valid (`self.get_camera` camera_id))
  (if (not _is_valid)
    (`KismetArrayLibrary.Array_Add` (`self.camera_list`) camera_id)
    (`KismetArrayLibrary.Array_Add` (`self.camera_component`) camera_component)))

(fn `get_auto_cam`
  (params (latest_cam :type Integer) (latest_interlocutor :type Name))
  (returns (random_cam :type "CineCameraComponent Object Reference") (latest_random :type Integer))
  (locals (local_random_value :type Integer :default 0) (local_latest_index :type Integer) (local_latest_interlocutor :type Name))
  ;[1 1 1] Get automatic cam.
  (set `local.local_latest_index` latest_cam)
  (set `local.local_latest_interlocutor` latest_interlocutor)
  (`|ExecutionSequence`
    (:`then_0`
      (switch `int` (`local.local_latest_index`)
        (:`Default`
          (set `local.local_random_value` (`KismetMathLibrary.RandomIntegerInRange` 0 2) :!label _label))
        (:`0`
          (goto _label))
        (:`1`
          (if (!= (`self.interlocutor_id`) (`local.local_latest_interlocutor`))
            (set `local.local_random_value` 2) ; this part of logic leads\nto keep the 180 rule of camera.
          ))
        (:`2`
          (if (!= (`self.interlocutor_id`) (`local.local_latest_interlocutor`))
            (set `local.local_random_value` 1) ; this part of logic leads\nto keep the 180 rule of camera.
          ))))
    (:`then_1`
      (return (`|GetArrayItem` (`|MakeArray` (`self.face_f`) (`self.face_l`) (`self.face_r`)) (`local.local_random_value`)) (`local.local_random_value`)))))

(fn `get_camera`
  (params (camera_id :type Name))
  (returns (is_valid :type Boolean) (found_index :type Integer) (camera_component :type "CameraComponent Object Reference"))
  (bind _returnvalue (`KismetArrayLibrary.Array_Find` (`self.camera_list`) camera_id))
  (bind _returnvalue_2 (>= _returnvalue 0))
  ;[1 1 1] Get camera component by id.
  (if _returnvalue_2
    (return _returnvalue_2 _returnvalue (`|GetArrayItem` (`self.camera_component`) _returnvalue))
    (else
      (return false 0 null))))

(fn `set_active_camera`
  (params (camera_id :type Name))
  (returns (camera_component :type "CameraComponent Object Reference") (is_valid :type Boolean))
  ;[1 1 1] Set specific found camera as active.
  (bind (_is_valid _found_index _camera_component) (`self.get_camera` camera_id))
  (if _is_valid
    (bind (_arrayindex _arrayelement) (`/Game/EditorBlueprintResources/StandardMacros.ReverseForEachLoop` (`self.camera_component`))
      (:`LoopBody`
        (`ActorComponent.SetActive` _arrayelement false false))
      (:`Completed`
        (`ActorComponent.SetActive` _camera_component true false)
        (return _camera_component true)))
    (else
      (return null false))))

(fn `UserConstructionScript`)