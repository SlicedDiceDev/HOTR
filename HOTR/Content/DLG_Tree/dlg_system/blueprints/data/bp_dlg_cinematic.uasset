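; Dialogue cinematic actor that plays a Level Sequence for a dialogue, looping or self-destroying at its end time.
; The sequence drives spawned proxy actors bound through a spawned cinematic object.
; Each tick copies proxy bone poses as snapshots to the real characters' anim instances, skipping the first frame against T-pose pops, and optionally applies ground-traced proxy transforms.
; A positioning mode only snaps actors into place, then destroys itself.
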(event `self.ReceiveTick`
  (params (DeltaSeconds :type "Float (single-precision)"))
  ;[1 1 1] DLG cinematic actor beginplay is here.
  (if (`self.is_started`)
    (if (not (`self.is_destroy`))
      (`self.tick_cinematic`)
      (`self.tick_proxy`))))

(event `destroy_cinematic`
  ;[1 1 1] This type of data needs delayed destroy as well for specific cases.
  (set `self.is_destroy` true)
  (`self.notify_cine_anim` false)
  (`|ExecutionSequence`
    (:`then_0`
      (`/Game/EditorBlueprintResources/StandardMacros.IsValid` (`self.active_sequencer`)
        (:`Is Valid`
          (`MovieSceneSequencePlayer.Pause` (`LevelSequenceActor.SequencePlayer` (`self.active_sequencer`)))
          (`self.K2_DestroyActor` (`self.active_sequencer`))
          (set `self.active_sequencer` null))))
    (:`then_1`
      (`/Game/EditorBlueprintResources/StandardMacros.IsValid` (`self.cinematic_obj`)
        (:`Is Valid`
          (`self.K2_DestroyActor` (`self.cinematic_obj`)))))
    (:`then_2`
      (`KismetSystemLibrary.Delay` 1.0)
      (`self.K2_DestroyActor`))))

(fn `bind_cinematic`
  (params (unbind :type Boolean))
  (locals (local_unbind :type Boolean))
  ;[1 1 1] Bind cinematic roles.
  (set `local.local_unbind` unbind)
  (`/Game/DLG_Tree/dlg_system/dialogue_objects/parents/object_dlg_cinematic_parent.init_object` (`self.cinematic_obj`) (`self.dlg_actor`) self (`self.cinematic_id`) (`local.local_unbind`)))

(fn `get_playback`
  (returns (ReturnValue :type "Float (double-precision)"))
  (bind (_frame _framerate) (`KismetMathLibrary.BreakQualifiedFrameTime` (`MovieSceneSequencePlayer.GetCurrentTime` (`LevelSequenceActor.SequencePlayer` (`self.active_sequencer`)))))
  ;[1 1 1] Get playback pos for other blueprints.
  (`/Game/EditorBlueprintResources/StandardMacros.IsValid` (`self.active_sequencer`)
    (:`Is Valid`
      (return (/ (`KismetMathLibrary.Conv_IntToDouble` (`.Value` (break `FrameNumber` _frame))) (`KismetMathLibrary.Conv_IntToDouble` (`KismetMathLibrary.BreakFrameRate` _framerate)))))
    (:`Is Not Valid`
      (return 0.0))))

(fn `init_cinematic`
  (params (dlg_actor :type "/Game/DLG_Tree/dlg_system/blueprints/base/bp_dlg_actor Object Reference") (cinematic_info :type "/Game/DLG_Tree/dlg_system/structs/05_cinematic/s_dlg_cinematic_info Structure") (start_time :type "Float (double-precision)") (positionate :type Boolean))
  ;[1 1 1] Init and start cinematic.
  (set `self.dlg_actor` dlg_actor)
  (set `self.cinematic_info` cinematic_info)
  (set `self.start_time` start_time)
  (set `self.is_positionate` positionate)
  (if (`KismetSystemLibrary.IsValidClass` (`.cinematic_class_31_474EC66648BC689EE829E886A7E4ACDE` (break `/Game/DLG_Tree/dlg_system/structs/05_cinematic/s_dlg_cinematic_info` (`self.cinematic_info`))))
    (bind _returnvalue (`|SpawnActorFromClass` (`.cinematic_class_31_474EC66648BC689EE829E886A7E4ACDE` (break `/Game/DLG_Tree/dlg_system/structs/05_cinematic/s_dlg_cinematic_info` (`self.cinematic_info`))) (`KismetMathLibrary.MakeTransform` (0.0 0.0 0.0)) "AlwaysSpawn" "SelectDefaultAtRuntime" self null))
    (set `self.cinematic_obj` _returnvalue)
    (`|ExecutionSequence`
      (:`then_0`
        (set `self.cinematic_anim` (`/Game/DLG_Tree/dlg_system/dialogue_objects/parents/object_dlg_cinematic_parent.cinematic_anims` (`self.cinematic_obj`)))
        (bind (_is_valid _cinematic_data) (`/Game/DLG_Tree/dlg_system/dialogue_objects/parents/object_dlg_cinematic_parent.get_cinematic` (`self.cinematic_obj`) (`self.cinematic_info`)))
        (if _is_valid
          (set `self.cinematic_data` _cinematic_data)
          (if (== (`self.start_time`) 0.0)
            (set `self.start_time` (`.start_time_5_202C86E54021DDD5D760C2BB4F014F07` (break `/Game/DLG_Tree/dlg_system/structs/05_cinematic/s_dlg_cinematic_list` (`self.cinematic_data`)))))))
      (:`then_1`
        (bind (_arrayindex _arrayelement) (`/Game/EditorBlueprintResources/StandardMacros.ReverseForEachLoop` (`self.cinematic_anim`))
          (:`LoopBody`
            (bind (_proxy_class _actor_id _actor_index) (break `/Game/DLG_Tree/dlg_system/structs/05_cinematic/s_dlg_cinematic_anim` _arrayelement))
            (if (>= (`KismetArrayLibrary.Array_Find` (`/Game/DLG_Tree/dlg_system/blueprints/base/bp_dlg_actor.actor_list` (`self.dlg_actor`)) _actor_id) 0)
              _
              (elif (`KismetArrayLibrary.Array_IsValidIndex` (`/Game/DLG_Tree/dlg_system/blueprints/base/bp_dlg_actor.actor_list` (`self.dlg_actor`)) _actor_index)
                (setmembers `/Game/DLG_Tree/dlg_system/structs/05_cinematic/s_dlg_cinematic_anim` :`StructRef` (`|GetArrayItem` (`self.cinematic_anim`) _arrayindex) :`actor_id` (`|GetArrayItem` (`/Game/DLG_Tree/dlg_system/blueprints/base/bp_dlg_actor.actor_list` (`self.dlg_actor`)) _actor_index)))))))
      (:`then_2`
        (if (`self.is_positionate`)
          (`self.set_pos`)
          (else
            (`self.start_cinematic`)))))
    (else
      (`self.destroy_cinematic`))))

(fn `notify_cine_anim`
  (params (enable :type Boolean))
  ;[1 1 1] Enable cinematic animation mode or disable it.
  (if enable
    (bind _array_element (`/Game/EditorBlueprintResources/StandardMacros.ForEachLoop` (`self.cinematic_anim`))
      (:`LoopBody`
        (bind (_is_valid _is_component_valid _actor_index _actor_reference _dlg_component) (`/Game/DLG_Tree/dlg_system/blueprints/base/bp_dlg_actor.get_dlg_actor` (`self.dlg_actor`) (`.actor_id_2_BEBEA7A647E336B14901FD9969150499` (break `/Game/DLG_Tree/dlg_system/structs/05_cinematic/s_dlg_cinematic_anim` _array_element))))
        (if _is_component_valid
          (`/Game/DLG_Tree/dlg_system/blueprints/base/bp_dlg_component.receive_anim_cinematic` _dlg_component (`self.dlg_actor`) (`self.cinematic_id`) true))))
    (else
      (bind _array_element_2 (`/Game/EditorBlueprintResources/StandardMacros.ForEachLoop` (`self.cinematic_anim`))
        (:`LoopBody`
          (bind (_is_valid_2 _is_component_valid_2 _actor_index_2 _actor_reference_2 _dlg_component_2) (`/Game/DLG_Tree/dlg_system/blueprints/base/bp_dlg_actor.get_dlg_actor` (`self.dlg_actor`) (`.actor_id_2_BEBEA7A647E336B14901FD9969150499` (break `/Game/DLG_Tree/dlg_system/structs/05_cinematic/s_dlg_cinematic_anim` _array_element_2))))
          (if _is_component_valid_2
            (`/Game/DLG_Tree/dlg_system/blueprints/base/bp_dlg_component.receive_anim_cinematic` _dlg_component_2 (`self.dlg_actor`) (`self.cinematic_id`) false)))))))

(fn `set_pos`
  (locals (local_data :type "/Game/DLG_Tree/dlg_system/structs/05_cinematic/s_dlg_cinematic_anim Structure") (local_id :type Name) (local_true_actor :type "Actor Object Reference") (local_proxy_base :type "/Game/DLG_Tree/dlg_system/blueprints/proxy/bp_dlg_proxy_base Object Reference"))
  (bind _local_proxy_base (`local.local_proxy_base`))
  ;[1 1 1] Fix actor positions and destroy cinematic.
  (bind _outactor (`LevelSequencePlayer.CreateLevelSequencePlayer` (`.cinematic_sequence_13_95A0CB9D419D0EE8BCBE279316FA7AB1` (break `/Game/DLG_Tree/dlg_system/structs/05_cinematic/s_dlg_cinematic_list` (`self.cinematic_data`))) (make `MovieSceneSequencePlaybackSettings` false (struct) 1.0 0.0 false false false false false false "None" false true)))
  (set `self.active_sequencer` _outactor)
  (`/Game/EditorBlueprintResources/StandardMacros.IsValid` (`self.active_sequencer`)
    (:`Is Valid`
      (`|ExecutionSequence`
        (:`then_0`
          (bind _array_element (`/Game/EditorBlueprintResources/StandardMacros.ForEachLoop` (`/Game/DLG_Tree/dlg_system/blueprints/base/bp_dlg_actor.actor_list` (`self.dlg_actor`)))
            (:`LoopBody`
              (switch `name` _array_element
                (:`Default`
                  (`/Game/DLG_Tree/dlg_system/blueprints/base/bp_dlg_actor.add_proxy` (`self.dlg_actor`) _array_element "/Game/DLG_Tree/dlg_system/blueprints/proxy/bp_dlg_proxy_base.bp_dlg_proxy_base_C" true))
                (:`dlg`
                  (bind _proxy_reference (`/Game/DLG_Tree/dlg_system/blueprints/base/bp_dlg_actor.add_proxy` (`self.dlg_actor`) "dlg" "/Game/DLG_Tree/dlg_system/blueprints/proxy/bp_dlg_proxy_base.bp_dlg_proxy_base_C" true))
                  (`self.K2_SetActorTransform` _proxy_reference (`self.GetTransform` (`self.dlg_actor`)) false false))))
            (:`Completed`
              (`self.bind_cinematic` false))))
        (:`then_1`
          (`MovieSceneSequencePlayer.SetPlaybackPosition` :`self` (`LevelSequenceActor.SequencePlayer` (`self.active_sequencer`)))
          (`MovieSceneSequencePlayer.SetTimeRange` (`LevelSequenceActor.SequencePlayer` (`self.active_sequencer`)) 0.0 9999999.0))
        (:`then_2`
          (`MovieSceneSequencePlayer.Pause` (`LevelSequenceActor.SequencePlayer` (`self.active_sequencer`)))
          (bind _array_element_2 (`/Game/EditorBlueprintResources/StandardMacros.ForEachLoop` (`/Game/DLG_Tree/dlg_system/blueprints/base/bp_dlg_actor.actor_list` (`self.dlg_actor`)))
            (:`LoopBody`
              (bind (_is_valid _is_component_valid _actor_index _actor_reference) (`/Game/DLG_Tree/dlg_system/blueprints/base/bp_dlg_actor.get_dlg_actor` (`self.dlg_actor`) _array_element_2))
              (if _is_component_valid
                (set `local.local_true_actor` _actor_reference)
                (bind (_is_valid_2 _found_index _proxy_actor) (`/Game/DLG_Tree/dlg_system/blueprints/base/bp_dlg_actor.get_proxy` (`self.dlg_actor`) _array_element_2))
                (if _is_valid_2
                  (set `local.local_proxy_base` _proxy_actor)
                  (`/Game/EditorBlueprintResources/StandardMacros.IsValid` (`local.local_proxy_base`)
                    (:`Is Valid`
                      (if (`self.ActorHasTag` (`local.local_proxy_base`) "cinematic_bind")
                        (bind _new_transform (`self.track_ground_z` (`local.local_true_actor`) (`self.GetTransform` (`local.local_proxy_base`)) true (`/Game/DLG_Tree/dlg_system/blueprints/proxy/bp_dlg_proxy_base.track_ground` _local_proxy_base) (`/Game/DLG_Tree/dlg_system/blueprints/proxy/bp_dlg_proxy_base.capsule_height` _local_proxy_base) (`/Game/DLG_Tree/dlg_system/blueprints/proxy/bp_dlg_proxy_base.capsule_radius` _local_proxy_base)))
                        (`self.K2_SetActorTransform` (`local.local_true_actor`) _new_transform false false)))))))
            (:`Completed`
              (`self.destroy_cinematic`))))))))

(fn `snapshot_data`
  (params (skeletal_mesh :type "SkeletalMeshComponent Object Reference"))
  (returns (snapshot_data :type "PoseSnapshot Structure"))
  (locals (local_mesh :type "SkeletalMeshComponent Object Reference") (local_name :type "Array of Name") (local_transform :type "Array of Transform Structure"))
  (bind _returnvalue (`KismetStringLibrary.Conv_StringToName` (`KismetSystemLibrary.GetDisplayName` (`local.local_mesh`))))
  ;[1 1 1] Snapshot all bones of the input mesh, and return as snapshot data.
  (bind _output_get (set `local.local_mesh` skeletal_mesh))
  (`/Game/EditorBlueprintResources/StandardMacros.IsValid` _output_get
    (:`Is Valid`
      (set `local.local_name` (`SceneComponent.GetAllSocketNames` (`local.local_mesh`)))
      (bind _array_element (`/Game/EditorBlueprintResources/StandardMacros.ForEachLoop` (`local.local_name`))
        (:`LoopBody`
          (`KismetArrayLibrary.Array_Add` (`local.local_transform`) (`SceneComponent.GetSocketTransform` (`local.local_mesh`) _array_element "RTS_ParentBoneSpace")))
        (:`Completed`
          (return (make `PoseSnapshot` (`local.local_transform`) (`local.local_name`) _returnvalue _returnvalue true)))))))

(fn `spawn_proxy`
  (locals (local_proxy_mesh :type "/Game/DLG_Tree/dlg_system/blueprints/proxy/bp_dlg_proxy_mesh Object Reference") (local_true_actor :type "Actor Object Reference") (local_id :type Name) (local_true_mesh :type "SkeletalMeshComponent Object Reference") (local_proxy_base :type "/Game/DLG_Tree/dlg_system/blueprints/proxy/bp_dlg_proxy_base Object Reference") (local_true_component :type "/Game/DLG_Tree/dlg_system/blueprints/base/bp_dlg_component Object Reference") (local_widget_parent :type "SceneComponent Object Reference"))
  (bind _mesh_list (`/Game/DLG_Tree/dlg_system/blueprints/base/bp_dlg_component.mesh_list` (`local.local_true_component`)))
  ;[1 1 1] Spawn role actors.
  (`|ExecutionSequence`
    (:`then_0`
      (bind _proxy_reference (`/Game/DLG_Tree/dlg_system/blueprints/base/bp_dlg_actor.add_proxy` (`self.dlg_actor`) "dlg" "/Game/DLG_Tree/dlg_system/blueprints/proxy/bp_dlg_proxy_base.bp_dlg_proxy_base_C" true))
      (`self.K2_SetActorTransform` _proxy_reference (`self.GetTransform` (`self.dlg_actor`)) false false)
      (`/Game/DLG_Tree/dlg_system/blueprints/data/bp_dlg_cut.spawn_cam_list` (`/Game/DLG_Tree/dlg_system/blueprints/base/bp_dlg_actor.dlg_cut` (`self.dlg_actor`))))
    (:`then_1`
      (bind (_array_element _array_index) (`/Game/EditorBlueprintResources/StandardMacros.ForEachLoop` (`/Game/DLG_Tree/dlg_system/blueprints/base/bp_dlg_actor.widget_actors` (`self.dlg_actor`)))
        (:`LoopBody`
          (`|ExecutionSequence`
            (:`then_0`
              (bind (_is_valid _widget_proxy) (`/Game/DLG_Tree/dlg_system/blueprints/data/bp_dlg_layout_widget_3d.get_widget_proxy` _array_element))
              (if _is_valid
                (set `local.local_widget_parent` (`SceneComponent.GetAttachParent` (`/Game/DLG_Tree/dlg_system/blueprints/proxy/bp_dlg_proxy_base.arrow_root` _widget_proxy)))
                (else
                  (set `local.local_widget_parent` null))))
            (:`then_1`
              (bind _widget_proxy_2 (`/Game/DLG_Tree/dlg_system/blueprints/base/bp_dlg_actor.add_widget_proxy` (`self.dlg_actor`) _array_index))
              (`/Game/EditorBlueprintResources/StandardMacros.IsValid` (`local.local_widget_parent`)
                (:`Is Valid`
                  (`self.K2_AttachToComponent` _widget_proxy_2 (`local.local_widget_parent`) "None" "KeepRelative" "KeepRelative" "KeepRelative" true))
                (:`Is Not Valid`
                  (`self.K2_SetActorTransform` _widget_proxy_2 (`self.GetTransform` _array_element) false false))))))))
    (:`then_2`
      (bind _array_element_2 (`/Game/EditorBlueprintResources/StandardMacros.ForEachLoop` (`self.cinematic_anim`))
        (:`LoopBody`
          (bind (_proxy_class _actor_id) (break `/Game/DLG_Tree/dlg_system/structs/05_cinematic/s_dlg_cinematic_anim` _array_element_2))
          (set `local.local_id` _actor_id)
          (bind (_is_valid_2 _is_component_valid _actor_index _actor_reference _dlg_component) (`/Game/DLG_Tree/dlg_system/blueprints/base/bp_dlg_actor.get_dlg_actor` (`self.dlg_actor`) (`local.local_id`)))
          (if _is_component_valid
            (set `local.local_true_actor` _actor_reference)
            (set `local.local_true_component` _dlg_component)
            (if (`KismetSystemLibrary.IsValidClass` _proxy_class)
              (bind _proxy_reference_2 (`/Game/DLG_Tree/dlg_system/blueprints/base/bp_dlg_actor.add_proxy` (`self.dlg_actor`) (`local.local_id`) _proxy_class true))
              (set `local.local_proxy_base` _proxy_reference_2)
              (else
                (bind _proxy_reference_3 (`/Game/DLG_Tree/dlg_system/blueprints/base/bp_dlg_actor.add_proxy` (`self.dlg_actor`) (`local.local_id`) "/Game/DLG_Tree/dlg_system/blueprints/proxy/bp_dlg_proxy_base.bp_dlg_proxy_base_C" true))
                (set `local.local_proxy_base` _proxy_reference_3)))
            (`self.K2_SetActorTransform` (`local.local_proxy_base`) (`self.GetTransform` (`local.local_true_actor`)) false false)
            (`/Game/EditorBlueprintResources/StandardMacros.IsValid` (`local.local_proxy_base`)
              (:`Is Valid`
                (`|ExecutionSequence`
                  (:`then_0`
                    (bind _array_element_3 (`/Game/EditorBlueprintResources/StandardMacros.ForEachLoop` (`/Game/DLG_Tree/dlg_system/blueprints/base/bp_dlg_component.mesh_list` (`local.local_true_component`)))
                      (:`LoopBody`
                        (bind _snapshot_data (`self.snapshot_data` _array_element_3))
                        (message `/Game/DLG_Tree/dlg_system/blueprints/proxy/bp_proxy_interface.receive_snapshot` (`SkeletalMeshComponent.GetAnimInstance` _array_element_3) _snapshot_data))))
                  (:`then_1`
                    (bind (_array_element_4 _array_index_2) (`/Game/EditorBlueprintResources/StandardMacros.ForEachLoop` (`/Game/DLG_Tree/dlg_system/blueprints/proxy/bp_dlg_proxy_base.mesh_list` (`local.local_proxy_base`)))
                      (:`LoopBody`
                        (if (`KismetArrayLibrary.Array_IsValidIndex` _mesh_list _array_index_2)
                          (bind _snapshot_data_2 (`self.snapshot_data` (`|GetArrayItem` _mesh_list _array_index_2)))
                          (message `/Game/DLG_Tree/dlg_system/blueprints/proxy/bp_proxy_interface.receive_snapshot` (`SkeletalMeshComponent.GetAnimInstance` _array_element_4) _snapshot_data_2))))))))))))))

(fn `start_cinematic`
  (bind (_is_loop _cinematic_id _start_time _end_time) (break `/Game/DLG_Tree/dlg_system/structs/05_cinematic/s_dlg_cinematic_list` (`self.cinematic_data`)))
  (bind (_frame _framerate) (`KismetMathLibrary.BreakQualifiedFrameTime` (`MovieSceneSequencePlayer.GetEndTime` (`LevelSequenceActor.SequencePlayer` (`self.active_sequencer`)))))
  ;[1 1 1] Start cinematic logic.
  (`/Game/DLG_Tree/dlg_system/blueprints/base/bp_dlg_actor.remove_proxy` (`self.dlg_actor`) "None" true)
  (`/Game/EditorBlueprintResources/StandardMacros.IsValid` (`self.active_sequencer`)
    (:`Is Valid`
      (`LevelSequenceActor.SetSequence` (`self.active_sequencer`) (`.cinematic_sequence_13_95A0CB9D419D0EE8BCBE279316FA7AB1` (break `/Game/DLG_Tree/dlg_system/structs/05_cinematic/s_dlg_cinematic_list` (`self.cinematic_data`)))))
    (:`Is Not Valid`
      (bind _outactor (`LevelSequencePlayer.CreateLevelSequencePlayer` (`.cinematic_sequence_13_95A0CB9D419D0EE8BCBE279316FA7AB1` (break `/Game/DLG_Tree/dlg_system/structs/05_cinematic/s_dlg_cinematic_list` (`self.cinematic_data`))) (make `MovieSceneSequencePlaybackSettings` false (struct) 1.0 0.0 false false false false false false "None" false true)))
      (set `self.active_sequencer` _outactor)))
  (`/Game/EditorBlueprintResources/StandardMacros.IsValid` (`self.active_sequencer`)
    (:`Is Valid`
      (`|ExecutionSequence`
        (:`then_0`
          (`self.spawn_proxy`)
          (`self.bind_cinematic` false)
          (`self.notify_cine_anim` true))
        (:`then_1`
          (`/Game/EditorBlueprintResources/StandardMacros.IsValid` (`self.cinematic_obj`)
            (:`Is Valid`
              (set `self.playback_start` (`self.start_time`))
              (set `self.playback_end` (/ (`KismetMathLibrary.Conv_IntToDouble` (`.Value` (break `FrameNumber` _frame))) (`KismetMathLibrary.Conv_IntToDouble` (`KismetMathLibrary.BreakFrameRate` _framerate))))
              (`MovieSceneSequencePlayer.SetPlaybackPosition` (`LevelSequenceActor.SequencePlayer` (`self.active_sequencer`)) (make `MovieSceneSequencePlaybackParams` (struct :`FrameNumber` (struct)) (`self.start_time`) "" (struct) "Time" "Jump"))
              (`MovieSceneSequencePlayer.SetTimeRange` (`LevelSequenceActor.SequencePlayer` (`self.active_sequencer`)) (`self.start_time`) 9999999.0)
              (if (!= _end_time 0.0)
                (set `self.playback_end` _end_time)))))
        (:`then_2`
          (`MovieSceneSequencePlayer.Play` (`LevelSequenceActor.SequencePlayer` (`self.active_sequencer`)))
          (set `self.is_started` true)
          (`self.tick_proxy`))))))

(fn `stop_cinematic`
  ;[1 1 1] Stop cinematic.
  (set `self.is_started` false)
  (`/Game/EditorBlueprintResources/StandardMacros.IsValid` (`self.cinematic_obj`)
    (:`Is Valid`
      (`|ExecutionSequence`
        (:`then_0`
          (`/Game/EditorBlueprintResources/StandardMacros.IsValid` (`self.active_sequencer`)
            (:`Is Valid`
              (`MovieSceneSequencePlayer.Pause` (`LevelSequenceActor.SequencePlayer` (`self.active_sequencer`)))
              (`self.K2_DestroyActor` (`self.active_sequencer`))
              (set `self.active_sequencer` null))))
        (:`then_1`
          (if (`.is_loop_1_7C024F634473D4626F2FAAB480F49E5B` (break `/Game/DLG_Tree/dlg_system/structs/05_cinematic/s_dlg_cinematic_list` (`self.cinematic_data`)))
            (if (not (`self.is_destroy`))
              (`self.start_cinematic`))
            (else
              (`self.destroy_cinematic`))))))))

(fn `synchronize_cinematic`
  (params (playback_time :type "Float (double-precision)"))
  ;[1 1 1] Synch for dialogues.
  (`/Game/EditorBlueprintResources/StandardMacros.IsValid` (`self.active_sequencer`)
    (:`Is Valid`
      (`MovieSceneSequencePlayer.SetPlaybackPosition` (`LevelSequenceActor.SequencePlayer` (`self.active_sequencer`)) (make `MovieSceneSequencePlaybackParams` (struct :`FrameNumber` (struct)) playback_time "" (struct) "Time"))
      (`self.tick_proxy`)
      (`self.tick_cinematic`))))

(fn `tick_cinematic`
  (bind (_frame _framerate) (`KismetMathLibrary.BreakQualifiedFrameTime` (`MovieSceneSequencePlayer.GetCurrentTime` (`LevelSequenceActor.SequencePlayer` (`self.active_sequencer`)))))
  ;[1 1 1] Tick cinematic sequence.
  (`/Game/EditorBlueprintResources/StandardMacros.IsValid` (`self.active_sequencer`)
    (:`Is Valid`
      (if (>= (/ (`KismetMathLibrary.Conv_IntToDouble` (`.Value` (break `FrameNumber` _frame))) (`KismetMathLibrary.Conv_IntToDouble` (`KismetMathLibrary.BreakFrameRate` _framerate))) (`self.playback_end`))
        (`self.stop_cinematic`)))
    (:`Is Not Valid`
      (`self.destroy_cinematic`))))

(fn `tick_proxy`
  (locals (local_true_actor :type "Actor Object Reference") (local_proxy_base :type "/Game/DLG_Tree/dlg_system/blueprints/proxy/bp_dlg_proxy_base Object Reference") (local_data :type "/Game/DLG_Tree/dlg_system/structs/05_cinematic/s_dlg_cinematic_anim Structure") (local_true_component :type "/Game/DLG_Tree/dlg_system/blueprints/base/bp_dlg_component Object Reference") (local_proxy_mesh :type "/Game/DLG_Tree/dlg_system/blueprints/proxy/bp_dlg_proxy_mesh Object Reference"))
  (bind _local_proxy_base (`local.local_proxy_base`))
  (bind (_proxy_class _actor_id _actor_index _tick_transform _use_sweep) (break `/Game/DLG_Tree/dlg_system/structs/05_cinematic/s_dlg_cinematic_anim` (`local.local_data`)))
  (bind (_proxy_class_2 _actor_id_2) (break `/Game/DLG_Tree/dlg_system/structs/05_cinematic/s_dlg_cinematic_anim` (`local.local_data`)))
  (bind _mesh_list (`/Game/DLG_Tree/dlg_system/blueprints/base/bp_dlg_component.mesh_list` (`local.local_true_component`)))
  ;[1 1 1] Send char animation data to owner.
  (`/Game/EditorBlueprintResources/StandardMacros.IsValid` (`self.active_sequencer`)
    (:`Is Valid`
      (if (`self.is_started`)
        (bind _array_element (`/Game/EditorBlueprintResources/StandardMacros.ForEachLoop` (`self.cinematic_anim`))
          (:`LoopBody`
            (set `local.local_data` _array_element)
            (bind (_is_valid _is_component_valid _actor_index_2 _actor_reference _dlg_component) (`/Game/DLG_Tree/dlg_system/blueprints/base/bp_dlg_actor.get_dlg_actor` (`self.dlg_actor`) _actor_id_2))
            (if _is_component_valid
              (set `local.local_true_actor` _actor_reference)
              (set `local.local_true_component` _dlg_component)
              (bind (_is_valid_2 _found_index _proxy_actor) (`/Game/DLG_Tree/dlg_system/blueprints/base/bp_dlg_actor.get_proxy` (`self.dlg_actor`) _actor_id_2))
              (if _is_valid_2
                (set `local.local_proxy_base` _proxy_actor)
                (`/Game/EditorBlueprintResources/StandardMacros.IsValid` (`local.local_proxy_base`)
                  (:`Is Valid`
                    (if (`self.ActorHasTag` (`local.local_proxy_base`) "cinematic_bind")
                      (`|ExecutionSequence`
                        (:`then_0`
                          (bind (_array_element_2 _array_index) (`/Game/EditorBlueprintResources/StandardMacros.ForEachLoop` (`/Game/DLG_Tree/dlg_system/blueprints/proxy/bp_dlg_proxy_base.mesh_list` (`local.local_proxy_base`)))
                            (:`LoopBody`
                              (bind _snapshot_data (`self.snapshot_data` _array_element_2))
                              (if (`KismetArrayLibrary.Array_IsValidIndex` _mesh_list _array_index)
                                (if (> (`self.GetGameTimeSinceCreation` (`local.local_proxy_base`)) (`GameplayStatics.GetWorldDeltaSeconds`))
                                  (message `/Game/DLG_Tree/dlg_system/blueprints/proxy/bp_proxy_interface.receive_snapshot` (`SkeletalMeshComponent.GetAnimInstance` (`|GetArrayItem` _mesh_list _array_index)) _snapshot_data))))))
                        (:`then_1`
                          (if _tick_transform
                            (bind _new_transform (`self.track_ground_z` (`local.local_true_actor`) (`self.GetTransform` (`local.local_proxy_base`)) _use_sweep (`/Game/DLG_Tree/dlg_system/blueprints/proxy/bp_dlg_proxy_base.track_ground` _local_proxy_base) (`/Game/DLG_Tree/dlg_system/blueprints/proxy/bp_dlg_proxy_base.capsule_height` _local_proxy_base) (`/Game/DLG_Tree/dlg_system/blueprints/proxy/bp_dlg_proxy_base.capsule_radius` _local_proxy_base)))
                            (`self.K2_SetActorTransform` (`local.local_true_actor`) _new_transform false false)))))))))))))))

(fn `track_ground_z`
  (params (base_actor :type "Actor Object Reference") (target_transform :type "Transform Structure") (use_sweep :type Boolean) (track_ground_z :type "Float (double-precision)") (capsule_height :type "Float (double-precision)") (capsule_radius :type "Float (double-precision)"))
  (returns (new_transform :type "Transform Structure"))
  (locals (local_actor :type "Actor Object Reference") (local_new_location :type "Vector Structure") (local_proxy_location :type "Vector Structure" :default (0.0 0.0 0.0)) (local_capsule_height :type "Float (double-precision)" :default 0.0) (local_target_transform :type "Transform Structure") (local_track_z :type "Float (double-precision)") (local_above_z :type "Float (double-precision)") (local_start_transform :type "Transform Structure") (local_sweep :type Boolean) (local_capsule_rad :type "Float (double-precision)"))
  ;[1 1 1] Auto-Track ground level for cinematic actors,
  ; so for example if cutscene does have flat ground, and dynamic cutscene may have different ground,
  ; so characters and objects will be not floating in air,
  ; thus this logic should track the ground and align all the objects by their default ground level.
  (set `local.local_actor` base_actor)
  (set `local.local_start_transform` (`self.GetTransform` (`local.local_actor`)))
  (set `local.local_target_transform` target_transform)
  (set `local.local_sweep` use_sweep)
  (set `local.local_track_z` track_ground_z)
  (set `local.local_above_z` capsule_height)
  (set `local.local_capsule_rad` capsule_radius)
  (set `local.local_proxy_location` (.location (`local.local_target_transform`)))
  (`|ExecutionSequence`
    (:`then_0`
      (`|ExecutionSequence`
        (:`then_0`
          (if (`local.local_sweep`)
            (bind (_outhit _returnvalue) (`KismetSystemLibrary.SphereTraceSingleForObjects` (.location (`local.local_start_transform`)) (`local.local_proxy_location`) (`local.local_capsule_rad`) (`|MakeArray` "ObjectTypeQuery1" :!type "EObjectTypeQuery Enum")))
            (if _returnvalue
              (set `local.local_proxy_location` (`.Location` (`GameplayStatics.BreakHitResult` _outhit))))))
        (:`then_1`
          (if (!= (`local.local_track_z`) 0.0)
            (bind (_outhit_2 _returnvalue_2) (`KismetSystemLibrary.SphereTraceSingleForObjects` (`local.local_proxy_location`) (+ (`local.local_proxy_location`) (* (`self.GetActorUpVector` (`local.local_actor`)) (* (`KismetMathLibrary.Abs` (+ (`local.local_track_z`) (`local.local_above_z`))) -1.0))) 1.0 (`|MakeArray` "ObjectTypeQuery1" :!type "EObjectTypeQuery Enum")))
            (if _returnvalue_2
              (set `local.local_new_location` (+ (`.Location` (`GameplayStatics.BreakHitResult` _outhit_2)) (`KismetMathLibrary.MakeVector` 0.0 0.0 (`local.local_above_z`))))
              (else
                (set `local.local_new_location` (`local.local_proxy_location`))))
            (else
              (set `local.local_new_location` (`local.local_proxy_location`)))))))
    (:`then_1`
      (return (`KismetMathLibrary.MakeTransform` (`local.local_new_location`) (.rotation (`local.local_target_transform`)) (.scale (`local.local_target_transform`)))))))

(fn `UserConstructionScript`)