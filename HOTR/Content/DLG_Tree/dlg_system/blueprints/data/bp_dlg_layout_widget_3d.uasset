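; Dialogue layout actor that shows choice widgets either on the 2D screen layout or on front and back 3D widget components.
; Data table settings pick the mode, filling a widget list that receives init, clear, input, accept and fade calls.
; Each tick it follows a proxy actor's transform with optional interpolation and camera-facing rotation.
; It also reads the proxy's scale variable, so Sequencer can animate the widget through the proxy.
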(event `self.ReceiveTick`
  (params (DeltaSeconds :type "Float (single-precision)"))
  ;[1 1 1] Layout widget 3d/2d controller,
  ; Beginplay is here.
  (`/Game/EditorBlueprintResources/StandardMacros.IsValid` (`self.dlg_actor`)
    (:`Is Valid`
      (if (`self.is_started`)
        (if (not (`self.is_destroying`))
          (`self.tick_proxy_transform` (`.transform_interp_5_302CA7D5430506659F0BB38DCFC5B00F` (break `/Game/DLG_Tree/dlg_system/structs/07_widget/s_dlg_widget_settings_info` (`self.widget_settings`)))))))))

(event `delayed_destroy`
  ;[1 1 1] Delayed destroy event.
  (set `self.is_destroying` true)
  (`self.clear_widget`)
  (`KismetSystemLibrary.Delay` 2.0)
  (`self.K2_DestroyActor`))

(fn `clear_widget`
  ;[1 1 1] Clear widget data.
  (bind _array_element (`/Game/EditorBlueprintResources/StandardMacros.ForEachLoop` (`self.widget_list`))
    (:`LoopBody`
      (`/Game/DLG_Tree/dlg_system/widgets/other/w_01_dlg_3d_layout.layout_clear_widgets` _array_element))))

(fn `get_slot_widget`
  (params (layout_index :type Integer) (widget_slot :type Integer))
  (returns (is_valid :type Boolean) (widget_reference :type "/Game/DLG_Tree/dlg_system/widgets/other/w_03_dlg_parent_input Object Reference"))
  ;[1 1 1] Get widget in specific child slot.
  (if (`KismetArrayLibrary.Array_IsValidIndex` (`self.widget_list`) layout_index)
    (bind (_is_valid _widget_reference) (`/Game/DLG_Tree/dlg_system/widgets/other/w_01_dlg_3d_layout.get_child_widget` (`|GetArrayItem` (`self.widget_list`) layout_index) widget_slot))
    (return _is_valid _widget_reference)
    (else
      (return false null))))

(fn `get_widget_proxy`
  (returns (is_valid :type Boolean) (widget_proxy :type "/Game/DLG_Tree/dlg_system/blueprints/proxy/bp_dlg_proxy_widget Object Reference"))
  ;[1 1 1] Return current widget proxy.
  (bind (_is_valid _found_index _widget_actor _widget_proxy) (`/Game/DLG_Tree/dlg_system/blueprints/base/bp_dlg_actor.get_widget` (`self.dlg_actor`) self 0))
  (if _is_valid
    (`/Game/EditorBlueprintResources/StandardMacros.IsValid` _widget_proxy
      (:`Is Valid`
        (return true _widget_proxy))
      (:`Is Not Valid`
        (return false null)))
    (else
      (return false null))))

(fn `init_2d_widgets`
  (params (`2d_widget` :type Boolean))
  ;[1 1 1] Init the 2d widget.
  (set `self.2d_widget` `2d_widget`)
  (`|ExecutionSequence`
    (:`then_0`
      (`KismetArrayLibrary.Array_Clear` (`self.widget_list`)))
    (:`then_1`
      (bind (_is_valid _layout_widget) (`/Game/DLG_Tree/dlg_system/blueprints/base/bp_dlg_component.get_layout_widget` (`/Game/DLG_Tree/dlg_system/blueprints/base/bp_dlg_actor.bp_owning_dlg_component` (`self.dlg_actor`))))
      (if _is_valid
        (`/Game/EditorBlueprintResources/StandardMacros.IsValid` _layout_widget
          (:`Is Valid`
            (bind (_is_valid_2 _found_index) (`/Game/DLG_Tree/dlg_system/blueprints/base/bp_dlg_actor.get_widget` (`self.dlg_actor`) self 0))
            (if _is_valid_2
              (bind (_is_valid_3 _widget_reference) (`/Game/DLG_Tree/dlg_system/widgets/base/w_01_dlg_2d_layout.get_child_layout` _layout_widget _found_index))
              (if _is_valid_3
                (if (`self.2d_widget`)
                  (`KismetArrayLibrary.Array_Add` (`self.widget_list`) _widget_reference)
                  (else
                    (`/Game/DLG_Tree/dlg_system/widgets/other/w_01_dlg_3d_layout.layout_clear_widgets` _widget_reference)))))))))
    (:`then_2`
      (`|ExecutionSequence`
        (:`then_0`
          (bind _asw_01_dlg_3d_layout (cast `/Game/DLG_Tree/dlg_system/widgets/other/w_01_dlg_3d_layout` (`WidgetComponent.GetUserWidgetObject` (`self.w_front`))))
          (if (`self.2d_widget`)
            (`/Game/DLG_Tree/dlg_system/widgets/other/w_01_dlg_3d_layout.layout_clear_widgets` _asw_01_dlg_3d_layout)
            (else
              (`KismetArrayLibrary.Array_Add` (`self.widget_list`) _asw_01_dlg_3d_layout))))
        (:`then_1`
          (bind _asw_01_dlg_3d_layout_2 (cast `/Game/DLG_Tree/dlg_system/widgets/other/w_01_dlg_3d_layout` (`WidgetComponent.GetUserWidgetObject` (`self.w_back`))))
          (if (`self.2d_widget`)
            (`/Game/DLG_Tree/dlg_system/widgets/other/w_01_dlg_3d_layout.layout_clear_widgets` _asw_01_dlg_3d_layout_2)
            (else
              (`KismetArrayLibrary.Array_Add` (`self.widget_list`) _asw_01_dlg_3d_layout_2))))))
    (:`then_3`
      (bind _array_element (`/Game/EditorBlueprintResources/StandardMacros.ForEachLoop` (`self.widget_list`))
        (:`LoopBody`
          (`/Game/DLG_Tree/dlg_system/widgets/other/w_01_dlg_3d_layout.init_3d_layout` _array_element self (`self.widget_base`)))))))

(fn `init_widget`
  (params (dlg_actor :type "/Game/DLG_Tree/dlg_system/blueprints/base/bp_dlg_actor Object Reference") (widget_base :type "/Game/DLG_Tree/dlg_system/structs/07_widget/s_dlg_widget_info Structure"))
  ;[1 1 1] Init widget actor logic.
  (set `self.dlg_actor` dlg_actor)
  (set `self.widget_base` widget_base)
  (set `self.player_camera` (`GameplayStatics.GetPlayerCameraManager` 0))
  (`|ExecutionSequence`
    (:`then_0`
      (bind _returnvalue (`|GetDataTableRow` (`self.widget_datatable`) (`.widget_data_65_7F46B3064DAA5B6FC3AC35B6FE7594B4` (break `/Game/DLG_Tree/dlg_system/structs/07_widget/s_dlg_widget_info` (`self.widget_base`))))
        (:`then`
          (set `self.widget_settings` (`.dlg_widget_3_97C0039D4A1838BFC13A6A81ADF2B97A` (break `/Game/DLG_Tree/dlg_system/structs/07_widget/s_dlg_widget_settings_base` _returnvalue)))
          (`self.init_2d_widgets` (`.2d_widget_9_6BE005F544B59CD0A7AF39903CCE3345` (break `/Game/DLG_Tree/dlg_system/structs/07_widget/s_dlg_widget_settings_info` (`self.widget_settings`))) :!label _label))
        (:`RowNotFound`
          (bind _returnvalue_2 (`|GetDataTableRow` (`self.widget_datatable`) "default_widget")
            (:`then`
              (set `self.widget_settings` (`.dlg_widget_3_97C0039D4A1838BFC13A6A81ADF2B97A` (break `/Game/DLG_Tree/dlg_system/structs/07_widget/s_dlg_widget_settings_base` _returnvalue_2)))
              (goto _label))
            (:`RowNotFound`
              (`self.init_2d_widgets` true))))))
    (:`then_1`
      (`self.tick_proxy_transform` 0.0)
      (set `self.is_started` true))))

(fn `init_widget_action`
  (params (choice_info :type "/Game/DLG_Tree/dlg_system/structs/03_choice/s_dlg_branch_choice_info Structure") (widget_action :type "/Game/DLG_Tree/dlg_system/structs/07_widget/s_dlg_widget_choice Structure") (last_index :type Integer))
  ;[1 1 1] Posses 2d widgets from layout, by actions.
  (bind _array_element (`/Game/EditorBlueprintResources/StandardMacros.ForEachLoop` (`self.widget_list`))
    (:`LoopBody`
      (`/Game/DLG_Tree/dlg_system/widgets/other/w_01_dlg_3d_layout.init_action` _array_element choice_info widget_action last_index))))

(fn `layout_accept_selection`
  (params (select_choice :type Name))
  ;[1 1 1] Activate both child choices like single widget.
  (bind _array_element (`/Game/EditorBlueprintResources/StandardMacros.ForEachLoop` (`self.widget_list`))
    (:`LoopBody`
      (`/Game/DLG_Tree/dlg_system/widgets/other/w_01_dlg_3d_layout.accept_visual` _array_element select_choice))
    (:`Completed`
      (`/Game/DLG_Tree/dlg_system/blueprints/base/bp_dlg_actor.select_choice` (`self.dlg_actor`) select_choice))))

(fn `layout_fade`
  ;[1 1 1] Choice accept layout.
  (bind _array_element (`/Game/EditorBlueprintResources/StandardMacros.ForEachLoop` (`self.widget_list`))
    (:`LoopBody`
      (`/Game/DLG_Tree/dlg_system/widgets/other/w_01_dlg_3d_layout.layout_fade_selections` _array_element))))

(fn `layout_input`
  (params (input_id :type Name) (is_pressed :type Boolean))
  (locals (local_input :type Name) (local_pressed :type Boolean))
  ;[1 1 1] Layout widget input.
  (set `local.local_input` input_id)
  (set `local.local_pressed` is_pressed)
  (if (`.selection_mode_12_FB9176E94709F7A2E47C59A33F6DF010` (break `/Game/DLG_Tree/dlg_system/structs/07_widget/s_dlg_widget_settings_info` (`self.widget_settings`)))
    (switch `name` (`local.local_input`)
      (:`dpad_u`
        (if (`local.local_pressed`)
          (bind _array_element (`/Game/EditorBlueprintResources/StandardMacros.ForEachLoop` (`self.widget_list`))
            (:`LoopBody`
              (`/Game/DLG_Tree/dlg_system/widgets/other/w_01_dlg_3d_layout.select_child` _array_element -1 false true)))))
      (:`dpad_d`
        (if (`local.local_pressed`)
          (bind _array_element_2 (`/Game/EditorBlueprintResources/StandardMacros.ForEachLoop` (`self.widget_list`))
            (:`LoopBody`
              (`/Game/DLG_Tree/dlg_system/widgets/other/w_01_dlg_3d_layout.select_child` _array_element_2 1 false true)))))
      (:`face_d`
        (if (not (`local.local_pressed`))
          (bind _array_element_3 (`/Game/EditorBlueprintResources/StandardMacros.ForEachLoop` (`self.widget_list`))
            (:`LoopBody`
              (`/Game/DLG_Tree/dlg_system/widgets/other/w_01_dlg_3d_layout.accept_child` _array_element_3 false 0))))))
    (elif (not (`local.local_pressed`))
      (bind _array_element_4 (`/Game/EditorBlueprintResources/StandardMacros.ForEachLoop` (`self.widget_list`))
        (:`LoopBody`
          (bind (_array_element_5 _array_index) (`/Game/EditorBlueprintResources/StandardMacros.ForEachLoop` (`/Game/DLG_Tree/dlg_system/widgets/other/w_01_dlg_3d_layout.widget_list` _array_element_4))
            (:`LoopBody`
              (if (== (`local.local_input`) (`.widget_input_id_30_1DB57D6F49F52D4565E55E816527F443` (break `/Game/DLG_Tree/dlg_system/structs/07_widget/s_dlg_widget_choice` (`/Game/DLG_Tree/dlg_system/widgets/other/w_03_dlg_parent_input.widget_action` _array_element_5))))
                (`/Game/DLG_Tree/dlg_system/widgets/other/w_01_dlg_3d_layout.select_child` _array_element_4 _array_index true true :!label _label)
                (`/Game/DLG_Tree/dlg_system/widgets/other/w_01_dlg_3d_layout.accept_child` _array_element_4 false 0)
                (elif (== (`local.local_input`) (`KismetStringLibrary.Conv_StringToName` (`KismetStringLibrary.Conv_IntToString` (`/Game/DLG_Tree/dlg_system/widgets/other/w_03_dlg_parent_input.widget_number` _array_element_5))))
                  (goto _label))))))))))

(fn `tick_proxy_transform`
  (params (interp_speed :type "Float (double-precision)"))
  (locals (local_speed :type "Float (double-precision)") (local_widget_proxy :type "/Game/DLG_Tree/dlg_system/blueprints/proxy/bp_dlg_proxy_widget Object Reference"))
  (bind (_transform_interp _rotation_interp _look_at_camera) (break `/Game/DLG_Tree/dlg_system/structs/07_widget/s_dlg_widget_settings_info` (`self.widget_settings`)))
  ;[1 1 1] Tick transform interp.
  (set `local.local_speed` interp_speed)
  (`|ExecutionSequence`
    (:`then_0`
      (bind (_is_valid _widget_proxy) (`self.get_widget_proxy`))
      (if _is_valid
        (set `local.local_widget_proxy` _widget_proxy)
        (`/Game/EditorBlueprintResources/StandardMacros.IsValid` (`local.local_widget_proxy`)
          (:`Is Valid`
            (set `self.latest_transform` (`self.GetTransform` (`local.local_widget_proxy`)))
            (bind _return_value (`/Game/DLG_Tree/dlg_system/blueprints/proxy/bp_dlg_proxy_base.get_float_var` (`local.local_widget_proxy`) "widget_scale"))
            (`self.update_widget_scale` _return_value)))))
    (:`then_1`
      (`self.K2_SetActorTransform` (`KismetMathLibrary.MakeTransform` (.location (`KismetMathLibrary.SelectTransform` (`KismetMathLibrary.TInterpTo` (`self.GetTransform`) (`self.latest_transform`) (`GameplayStatics.GetWorldDeltaSeconds`) (`local.local_speed`)) (`self.latest_transform`) (> (`local.local_speed`) 0.0))) (`KismetMathLibrary.SelectRotator` (`self.K2_GetActorRotation`) (.rotation (`KismetMathLibrary.SelectTransform` (`KismetMathLibrary.TInterpTo` (`self.GetTransform`) (`self.latest_transform`) (`GameplayStatics.GetWorldDeltaSeconds`) (`local.local_speed`)) (`self.latest_transform`) (> (`local.local_speed`) 0.0))) _look_at_camera)))
      (`self.tick_rotation_camera` _rotation_interp))))

(fn `tick_rotation_camera`
  (params (InterpSpeed :type "Float (double-precision)"))
  (locals (local_speed :type "Float (double-precision)"))
  (bind _yaw (.yaw (`self.K2_GetActorRotation` (`self.player_camera`))))
  (bind _returnvalue (`KismetMathLibrary.MakeRotator` 0.0 (`KismetMathLibrary.MapRangeClamped` (.pitch (`KismetMathLibrary.FindLookAtRotation` (`self.K2_GetActorLocation`) (`PlayerCameraManager.GetCameraLocation` (`self.player_camera`)))) -70.0 70.0 -90.0 90.0) (`KismetMathLibrary.SelectFloat` (`KismetMathLibrary.MapRangeClamped` _yaw 0.0 180.0 -180.0) (`KismetMathLibrary.MapRangeClamped` _yaw 0.0 -180.0 180.0) (> _yaw 0.0))))
  ;[1 1 1] Widget self rotate to face camera, by data.
  (set `local.local_speed` InterpSpeed)
  (`self.K2_SetActorRotation` (`KismetMathLibrary.SelectRotator` (`KismetMathLibrary.RInterpTo` (`self.K2_GetActorRotation`) _returnvalue (`GameplayStatics.GetWorldDeltaSeconds`) (`local.local_speed`)) _returnvalue (> (`local.local_speed`) 0.0))))

(fn `update_widget_scale`
  (params (widget_scale :type "Float (double-precision)"))
  ;[1 1 1] Update the widget scale.
  (set `self.widget_scale` widget_scale)
  (`SceneComponent.SetWorldScale3D` (`self.w_scale`) (`KismetMathLibrary.Conv_DoubleToVector` (`KismetMathLibrary.MapRangeUnclamped` (`self.widget_scale`) 0.1 1.0 0.1 0.3))))

(fn `UserConstructionScript`
  (`self.update_widget_scale` (`self.widget_scale`)))