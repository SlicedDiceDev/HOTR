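; 3D subtitle actor for the dialogue system that shows replies and speaker names on front and back widgets.
; InitDlgParent stores the owning dialogue component, caches the player camera manager and initializes both widgets, which later receive forwarded reply, name and clear calls.
; Each tick it snaps to face the camera, using yaw opposite the camera's and remapped look-at pitch, with optional interpolation left unused.
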(event `self.ReceiveBeginPlay`
  ;[1 1 1] 3d subtitles actor,
  ; beginplay is here.
)

(event `destroy_widget`
  ;[1 1 1] 3d subtitles actor,
  ; beginplay is here.
  (`self.K2_DestroyActor`))

(event `self.ReceiveTick`
  (params (DeltaSeconds :type "Float (single-precision)"))
  ;[1 1 1] 3d subtitles actor,
  ; beginplay is here.
  (`self.tick_rotation` 0.0))

(fn `clear_widget`
  (params (clear_quick :type Boolean))
  ;[1 1 1] Clear widgets logic.
  (bind _array_element (`/Game/EditorBlueprintResources/StandardMacros.ForEachLoop` (`self.subtitle_widgets`))
    (:`LoopBody`
      (`/Game/DLG_Tree/dlg_system/widgets/base/w_03_dlg_3d_subtitles.clear_visibility` _array_element clear_quick))))

(fn `init_dlg_parent`
  (params (bp_owner_dlg_component :type "/Game/DLG_Tree/dlg_system/blueprints/base/bp_dlg_component Object Reference"))
  ;[1 1 1] Init dlg parent, and attach to specific interlocutor.
  (set `self.bp_owning_dlg_component` bp_owner_dlg_component)
  (`|ExecutionSequence`
    (:`then_0`
      (`KismetArrayLibrary.Array_Clear` (`self.subtitle_widgets`))
      (set `self.player_camera` (`GameplayStatics.GetPlayerCameraManager` 0)))
    (:`then_1`
      (bind _array_element (`/Game/EditorBlueprintResources/StandardMacros.ForEachLoop` (`|MakeArray` (`self.w_front`) (`self.w_back`)))
        (:`LoopBody`
          (bind _asw_03_dlg_3d_subtitles (cast `/Game/DLG_Tree/dlg_system/widgets/base/w_03_dlg_3d_subtitles` (`WidgetComponent.GetUserWidgetObject` _array_element)))
          (`KismetArrayLibrary.Array_Add` (`self.subtitle_widgets`) _asw_03_dlg_3d_subtitles)
          (`/Game/DLG_Tree/dlg_system/widgets/base/w_03_dlg_3d_subtitles.init_widget` _asw_03_dlg_3d_subtitles self))))))

(fn `show_name`
  (params (name_id :type Name))
  ;[1 1 1] Show character's dialogue name
  (bind _array_element (`/Game/EditorBlueprintResources/StandardMacros.ForEachLoop` (`self.subtitle_widgets`))
    (:`LoopBody`
      (`/Game/DLG_Tree/dlg_system/widgets/base/w_03_dlg_3d_subtitles.show_name` _array_element name_id))))

(fn `tick_rotation`
  (params (interp_speed :type "Float (double-precision)"))
  (locals (local_speed :type "Float (double-precision)"))
  (bind _yaw (.yaw (`self.K2_GetActorRotation` (`self.player_camera`))))
  (bind _returnvalue (`KismetMathLibrary.MakeRotator` 0.0 (`KismetMathLibrary.MapRangeClamped` (.pitch (`KismetMathLibrary.FindLookAtRotation` (`self.K2_GetActorLocation`) (`PlayerCameraManager.GetCameraLocation` (`self.player_camera`)))) -70.0 70.0 -90.0 90.0) (`KismetMathLibrary.SelectFloat` (`KismetMathLibrary.MapRangeClamped` _yaw 0.0 180.0 -180.0) (`KismetMathLibrary.MapRangeClamped` _yaw 0.0 -180.0 180.0) (> _yaw 0.0))))
  ;[1 1 1] Tick and rotate subtitles widget to face player's camera.
  (set `local.local_speed` interp_speed)
  (`/Game/EditorBlueprintResources/StandardMacros.IsValid` (`self.player_camera`)
    (:`Is Valid`
      (`self.K2_SetActorRotation` (`KismetMathLibrary.SelectRotator` (`KismetMathLibrary.RInterpTo` (`self.K2_GetActorRotation`) _returnvalue (`GameplayStatics.GetWorldDeltaSeconds`) (`local.local_speed`)) _returnvalue (> (`local.local_speed`) 0.0))))))

(fn `update_reply`
  (params (reply_info :type "/Game/DLG_Tree/dlg_system/structs/02_reply/s_dlg_reply_info Structure") (dlg_actor :type "/Game/DLG_Tree/dlg_system/blueprints/base/bp_dlg_actor Object Reference"))
  ;[1 1 1] Send reply func.
  (set `self.latest_dlg_actor` dlg_actor)
  (bind _array_element (`/Game/EditorBlueprintResources/StandardMacros.ForEachLoop` (`self.subtitle_widgets`))
    (:`LoopBody`
      (`/Game/DLG_Tree/dlg_system/widgets/base/w_03_dlg_3d_subtitles.update_reply` _array_element reply_info (`self.latest_dlg_actor`)))))

(fn `UserConstructionScript`)